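; Side-scroller parallax camera actor that follows its owning character and scrolls layered background planes.
; On BeginPlay it sets X bounds, creates five dynamic materials, teleports to the owner and becomes the view target after a delay.
; Tick scales scrolling by owner direction and speed stat within bounds, driving four layers at different rates while clouds drift independently.
; The camera interpolates toward the clamped owner X, optionally following Z.
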(event `self.ReceiveBeginPlay`
  (bind _returnvalue (`self.GetTransform`))
  (bind _xasixofcam (`self.XAsixOfCam`))
  (bind (_returnvalue_x _returnvalue_y _returnvalue_z) (`KismetMathLibrary.BreakVector` (`self.K2_GetActorLocation` (`self.GetOwner`))))
  (bind _returnvalue_x_2 (`KismetMathLibrary.BreakVector` (`KismetMathLibrary.TransformLocation` _returnvalue (`|GetArrayItem` _xasixofcam 1))))
  (bind _returnvalue_x_3 (`KismetMathLibrary.BreakVector` (`KismetMathLibrary.TransformLocation` _returnvalue (`|GetArrayItem` _xasixofcam))))
  (`/Engine/EditorBlueprintResources/StandardMacros.IsValid` (`self.GetOwner`)
    (:`Is Valid`
      (`KismetSystemLibrary.PrintString` "parralax cam owner valid")
      (set `self.LeftX` _returnvalue_x_3)
      (set `self.Right X` _returnvalue_x_2)
      (`/Engine/EditorBlueprintResources/StandardMacros.IsValid` (`/Game/2DSideScrollerBP/Blueprints/BPF_2DSideScroller.FuncLibActorToCharacter` (`self.GetOwner`))
        (:`Is Valid`
          (bind _returnvalue_2 (`PrimitiveComponent.CreateDynamicMaterialInstance` (`self.Plane`) 0 "/Game/ParallaxCam/ParralaxMaterial1.ParralaxMaterial1" "None"))
          (set `self.DynamicMatInst` _returnvalue_2)
          (bind _returnvalue_3 (`PrimitiveComponent.CreateDynamicMaterialInstance` (`self.Plane1`) 0 "/Game/ParallaxCam/ParralaxMaterial2.ParralaxMaterial2" "None"))
          (set `self.Dynamic Mat Inst 2` _returnvalue_3)
          (bind _returnvalue_4 (`PrimitiveComponent.CreateDynamicMaterialInstance` (`self.Plane2`) 0 "/Game/ParallaxCam/ParralaxMaterial3.ParralaxMaterial3" "None"))
          (set `self.Dynamic Mat Inst 3` _returnvalue_4)
          (bind _returnvalue_5 (`PrimitiveComponent.CreateDynamicMaterialInstance` (`self.Plane3`) 0 "/Game/ParallaxCam/ParralaxMaterial4.ParralaxMaterial4" "None"))
          (set `self.Dynamic Mat Inst 4` _returnvalue_5)
          (bind _returnvalue_6 (`PrimitiveComponent.CreateDynamicMaterialInstance` (`self.Plane4`) 0 "/Game/ParallaxCam/ParralaxMaterial5.ParralaxMaterial5" "None"))
          (set `self.Dynamic Mat 5` _returnvalue_6)
          (`self.K2_TeleportTo` (+ (`self.offset`) (`KismetMathLibrary.MakeVector` _returnvalue_x 0.0 (+ _returnvalue_z 200.0))) (`self.K2_GetActorRotation`))
          (`KismetSystemLibrary.Delay` 1.0)
          (`PlayerController.SetViewTargetWithBlend` (`/Game/2DSideScrollerBP/Blueprints/BPF_2DSideScroller.FuncLibGetCharacterPlayerController` (`self.GetOwner`)) self 0.0 "VTBlend_Linear" 0.0 false))))))

(event `CamPositionUpdate`
  (bind (_returnvalue_x _returnvalue_y _returnvalue_z) (`KismetMathLibrary.BreakVector` (`self.K2_GetActorLocation`)))
  (bind _returnvalue (`GameplayStatics.GetWorldDeltaSeconds`))
  (bind (_returnvalue_x_2 _returnvalue_y_2 _returnvalue_z_2) (`KismetMathLibrary.BreakVector` (`self.K2_GetActorLocation` (`self.GetOwner`))))
  (bind _returnvalue_2 (`KismetMathLibrary.FClamp` _returnvalue_x_2 (`self.LeftX`) (`self.Right X`)))
  (`/Engine/EditorBlueprintResources/StandardMacros.IsValid` (`self.GetOwner`)
    (:`Is Valid`
      (if (`self.FollowZ`)
        (`self.K2_SetActorLocation` (`KismetMathLibrary.VInterpTo` (`self.K2_GetActorLocation`) (`KismetMathLibrary.MakeVector` _returnvalue_2 0.0 _returnvalue_z_2) _returnvalue 20.0))
        (else
          (`self.K2_SetActorLocation` (`KismetMathLibrary.VInterpTo` (`self.K2_GetActorLocation`) (`KismetMathLibrary.MakeVector` _returnvalue_2 0.0 _returnvalue_z) _returnvalue 20.0)))))))

(event `self.ReceiveTick`
  (params (DeltaSeconds :type "Float (single-precision)"))
  (bind _returnvalue_x (`KismetMathLibrary.BreakVector` (`self.K2_GetActorLocation` (`self.GetOwner`))))
  (bind _ascharacter (`/Game/2DSideScrollerBP/Blueprints/BPF_2DSideScroller.FuncLibActorToCharacter` (`self.GetOwner`)))
  (bind _returnvalue_x_2 (`KismetMathLibrary.BreakVector` (`self.GetVelocity` _ascharacter)))
  (bind (_stats_struct_var_charmaxhp _stats_struct_var_charcurrhp _stats_struct_var_charmaxmp _stats_struct_var_charcurrmp _stats_struct_var_attack _stats_struct_var_magicattack _stats_struct_var_def _stats_struct_var_magicdef _stats_struct_var_str _stats_struct_var_wisd _stats_struct_var_dex _stats_struct_var_luk _stats_struct_var_pur _stats_struct_var_vcs _stats_struct_var_boss _stats_struct_var_ied _stats_struct_var_evasion _stats_struct_var_accuracy _stats_struct_var_minrange _stats_struct_var_maxrange _stats_struct_var_speed) (break `/Game/GameSystem/Structures/CharactersStats_Struct` (`/Game/2DSideScrollerBP/Blueprints/2DSideScrollerCharacter.Stats_struct var` (`/Game/2DSideScrollerBP/Blueprints/BPF_2DSideScroller.FuncLibActorTo2DCharacter` (`self.GetOwner`)))))
  (bind _velocity_x (`KismetMathLibrary.BreakVector` (`MovementComponent.Velocity` (`Character.CharacterMovement` _ascharacter))))
  (set `self.deltaForClouds` (* (`KismetMathLibrary.VSize` (* (`KismetMathLibrary.Vector_Normal2D` (`KismetMathLibrary.MakeVector` 0.1)) (`self.BG_Speed`))) (`GameplayStatics.GetWorldDeltaSeconds`)))
  (if (not (or (< _returnvalue_x (`self.LeftX`)) (> _returnvalue_x (`self.Right X`))))
    (set `self.delta` (* (`GameplayStatics.GetWorldDeltaSeconds`) (`KismetMathLibrary.VSize` (* (`KismetMathLibrary.Vector_Normal2D` (`KismetMathLibrary.MakeVector` _returnvalue_x_2)) (/ (* (`self.BG_Speed`) (+ (/ (- (`KismetMathLibrary.Conv_IntToDouble` _stats_struct_var_speed) 100.0) 1.5) 100.0)) 100.0)))))
    (if (not (> _velocity_x 0.0))
      (bind _result (`/Engine/EditorBlueprintResources/StandardMacros.NegateFloat` (`self.delta`))
        (:`  `
          (bind _output_get (set `self.delta` _result)))))
    (bind _output_get_2 (set `self.CurrOffset` (+ (`self.CurrOffset`) _output_get)))
    (if (> _output_get_2 1.0)
      (bind _output_get_3 (set `self.CurrOffset` (`KismetMathLibrary.FMod` _output_get_2 1.0)))))
  (`MaterialInstanceDynamic.SetScalarParameterValue` (`self.DynamicMatInst`) "Offset" _output_get_3)
  (`MaterialInstanceDynamic.SetScalarParameterValue` (`self.Dynamic Mat Inst 2`) "Offset" (* (`self.CurrOffset`) 0.7))
  (`MaterialInstanceDynamic.SetScalarParameterValue` (`self.Dynamic Mat Inst 3`) "Offset" (* (`self.CurrOffset`) 0.5))
  (`MaterialInstanceDynamic.SetScalarParameterValue` (`self.Dynamic Mat Inst 4`) "Offset" (* (`self.CurrOffset`) 0.2))
  (bind _output_get_4 (set `self.CurrOffsetClouds` (+ (`self.deltaForClouds`) (`self.CurrOffsetClouds`))))
  (if (> _output_get_4 1.0)
    (set `self.CurrOffsetClouds` (`KismetMathLibrary.FMod` _output_get_4 1.0)))
  (`MaterialInstanceDynamic.SetScalarParameterValue` (`self.Dynamic Mat 5`) "Offset" _output_get_4)
  (`self.CamPositionUpdate`))

(fn `UserConstructionScript`)