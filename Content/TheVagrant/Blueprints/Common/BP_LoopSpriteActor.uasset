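; BP_LoopSpriteActor is a Paper2D actor that tiles one sprite into a grid on the X-Z plane.
; The construction script sets the base sprite and creates a dynamic material with adjustable hue, saturation and brightness.
; CalcOffset derives tile count and signed step per axis from start point, end point and spacing, treating zero spacing as a single tile.
; Spawned sprite components share that material and copy the base sprite's rotation, scale and collision profile.
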(fn `CalcOffset`
  (params (Start :type "Float (double-precision)") (End :type "Float (double-precision)") (Offset :type "Float (double-precision)"))
  (returns (LastIndex :type Integer) (Distance :type "Float (double-precision)"))
  (bind _returnvalue (- Start End))
  (if (!= Offset 0.0)
    (return (`KismetMathLibrary.FTrunc` (/ (`KismetMathLibrary.Abs` _returnvalue) Offset)) (* (`KismetMathLibrary.SignOfFloat` _returnvalue) Offset -1.0))
    (else
      (return 0 0.0))))

(fn `UserConstructionScript`
  (locals (DynamicMaterialVar :type "MaterialInstanceDynamic Object Reference"))
  (bind (_startpoint_x _startpoint_y _startpoint_z) (`KismetMathLibrary.BreakVector` (`self.StartPoint`)))
  (bind (_endpoint_x _endpoint_y _endpoint_z) (`KismetMathLibrary.BreakVector` (`self.EndPoint`)))
  (bind (_returnvalue_location _returnvalue_rotation _returnvalue_scale) (`KismetMathLibrary.BreakTransform` (`SceneComponent.GetRelativeTransform` (`self.PaperSprite`))))
  (bind (_lastindex _distance) (`self.CalcOffset` _startpoint_z _endpoint_z (`self.OffsetZ`)))
  (bind (_lastindex_2 _distance_2) (`self.CalcOffset` _startpoint_x _endpoint_x (`self.OffsetX`)))
  (`PaperSpriteComponent.SetSprite` (`self.PaperSprite`) (`self.NewSprite`))
  ;[1 1 1] Initialize Color
  (bind _returnvalue (`PrimitiveComponent.CreateDynamicMaterialInstance` (`self.PaperSprite`) 0 (`self.SourceMaterial`) "None"))
  (bind _output_get (set `local.DynamicMaterialVar` _returnvalue))
  (`MaterialInstanceDynamic.SetScalarParameterValue` _output_get "Hue" (`self.Hue`))
  (`MaterialInstanceDynamic.SetScalarParameterValue` _output_get "Saturation" (`self.Saturation`))
  (`MaterialInstanceDynamic.SetScalarParameterValue` _output_get "Brightness" (`self.Brightness`))
  ;[1 1 1] Add Sprite
  (for _index (range (+ _lastindex_2 1))
    (for _index_2 (range (+ _lastindex 1))
      (bind _returnvalue_2 (`AddComponent|NODE_AddPaperSpriteComponent-0` :`RelativeTransform` (`KismetMathLibrary.MakeTransform` (`KismetMathLibrary.MakeVector` (* _index _distance_2) 0.0 (* _index_2 _distance)) _returnvalue_rotation _returnvalue_scale)))
      ;[1 1 1] Set Sprite Color
      (`PaperSpriteComponent.SetSprite` _returnvalue_2 (`self.NewSprite`))
      (`PrimitiveComponent.SetMaterial` _returnvalue_2 0 (`local.DynamicMaterialVar`))
      (`PrimitiveComponent.SetCollisionProfileName` _returnvalue_2 (`PrimitiveComponent.GetCollisionProfileName` (`self.PaperSprite`)) true))))