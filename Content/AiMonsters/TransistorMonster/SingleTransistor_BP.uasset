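; Single Transistor monster, a flipbook-animated enemy that sets its stats in MonsterInfo on BeginPlay and wanders to random reachable points with pauses between moves.
; DmgTaken reduces hits by damage ignore offset by player IED, flags a miss at full ignore, and applies weakness, resistance and boss modifiers.
; Surviving hits lower HP and can trigger a hit flipbook; lethal hits call FreeMonster, which is empty, leaving the death flipbook unused.
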(event `self.ReceiveBeginPlay`
  (set `self.MonsterInfo` (make `/Game/InventorySystemAndWidgets/BluePrints/Structures/Struct_MonsterInfo` 10 10 2 5 3 "/Game/AiMonsters/TransistorMonster/BitMonster.BitMonster" "NewEnumerator8" "NewEnumerator7" "NewEnumerator8" 10 false 0 "Single Transistor" "/Game/AiMonsters/TransistorMonster/IdleTransistorFB.IdleTransistorFB" true false 100 0 3))
  (set `self.isMoving?` true :!label _label)
  (`|AIMoveTo` self null (`NavigationSystemV1.K2_GetRandomReachablePointInRadius` (`self.K2_GetActorLocation`) 500.0 null null) null
    (:`then`
      (set `self.isMoving?` false)
      (`KismetSystemLibrary.Delay` (`KismetMathLibrary.RandomFloatInRange` 2.0 5.0))
      (goto _label))))

(fn `DmgTaken`
  (params (`Dmg Received` :type Integer) (`Player IED` :type Integer) (`Player Attack Type` :type "/Game/InventorySystemAndWidgets/BluePrints/Enums/E_MonsterStrongOrWeekAgainst Enum" :default "NewEnumerator0") (`Boss Dmg %` :type Integer) (`Char REF` :type "/Game/2DSideScrollerBP/Blueprints/2DSideScrollerCharacter Object Reference"))
  (locals (`Miss?` :type Boolean) (`local %Dmg Ignored` :type "Float (double-precision)") (`Dmg Recieved` :type "Float (double-precision)") (localIsBoss :type Boolean) (`local player boss dmg%` :type Integer))
  (bind _returnvalue (`KismetMathLibrary.Conv_IntToDouble` `Dmg Received`))
  (bind _monsterinfo (`self.MonsterInfo`))
  (bind (_maxhp _currenthp _lvl _attackrating _defenserating _texture _type _resistanceto _weakagainst _damageignore _isboss_) (break `/Game/InventorySystemAndWidgets/BluePrints/Structures/Struct_MonsterInfo` (`self.MonsterInfo`)))
  (bind (_maxhp_2 _currenthp_2 _lvl_2 _attackrating_2 _defenserating_2 _texture_2 _type_2 _resistanceto_2 _weakagainst_2 _damageignore_2 _isboss__2 _magicattackrating _name _papersprite _canfly_ _canjump_ _speed _jump _exp _heal_ _knockbackofhp) (break `/Game/InventorySystemAndWidgets/BluePrints/Structures/Struct_MonsterInfo` _monsterinfo))
  (bind _returnvalue_2 (* (`KismetMathLibrary.Conv_IntToDouble` `Dmg Received`) 0.9))
  (bind _returnvalue_3 (* (`KismetMathLibrary.Conv_IntToDouble` `Dmg Received`) 1.1))
  (bind _returnvalue_4 (- _currenthp (`KismetMathLibrary.Round` (`local.Dmg Recieved`))))
  (bind _returnvalue_5 (- (`KismetMathLibrary.Conv_IntToDouble` _damageignore) (/ (`KismetMathLibrary.Conv_IntToDouble` (* _damageignore `Player IED`)) 100.0)))
  (set `local.local player boss dmg%` `Boss Dmg %`)
  (set `local.localIsBoss` _isboss_)
  ;[1 1 1] if the % dmg the monster ignores after calculation is greater than 100, the player does not have enouch %IED therefor cant hit the monster.
  (if (< _returnvalue_5 100.0)
    (set `local.local %Dmg Ignored` _returnvalue_5)
    (if (or (`|EnumEquality` _weakagainst `Player Attack Type`) (`|EnumEquality` _weakagainst "NewEnumerator8"))
      (set `local.Dmg Recieved` (- _returnvalue_3 (/ (* (`local.local %Dmg Ignored`) _returnvalue_3) 100.0)))
      (elif (or (`|EnumEquality` _resistanceto `Player Attack Type`) (`|EnumEquality` _resistanceto "NewEnumerator8"))
        (set `local.Dmg Recieved` (- _returnvalue_2 (/ (* (`local.local %Dmg Ignored`) _returnvalue_2) 100.0)))
        (else
          (set `local.Dmg Recieved` (- _returnvalue (/ (* (`local.local %Dmg Ignored`) _returnvalue) 100.0))) ; not strong or weak against the attack type
        )))
    (if (`local.localIsBoss`)
      (set `local.Dmg Recieved` (/ (* (`local.Dmg Recieved`) (`KismetMathLibrary.Conv_IntToDouble` (`local.local player boss dmg%`))) 100.0)))
    (if (<= _returnvalue_4 0)
      (`self.Free Monster` `Char REF`)
      (else
        (bind _structout (setmembers `/Game/InventorySystemAndWidgets/BluePrints/Structures/Struct_MonsterInfo` :`StructRef` _monsterinfo :`CurrentHP` _returnvalue_4))
        (set `self.MonsterInfo` _structout)
        (if (>= (/ (* (`local.Dmg Recieved`) (`KismetMathLibrary.Conv_IntToDouble` _maxhp_2)) 100.0) (`KismetMathLibrary.Conv_IntToDouble` _knockbackofhp))
          (`PaperFlipbookComponent.SetFlipbook` (`self.Sprite Flipbook`) "/Game/AiMonsters/TransistorMonster/TransistorBeingHitFB.TransistorBeingHitFB"))))
    (else
      (set `local.Miss?` true))))

(fn `Free Monster`
  (params (`Char REF` :type "/Game/2DSideScrollerBP/Blueprints/2DSideScrollerCharacter Object Reference")))

(fn `UserConstructionScript`)