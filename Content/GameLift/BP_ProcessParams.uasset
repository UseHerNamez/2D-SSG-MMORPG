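; GameLift process parameters Blueprint that handles server process callbacks for game session start, update, termination and health checks.
; On session start it runs the parent handler, then scans the game properties for the map key and broadcasts its value as a level name through the OnOpenLevel dispatcher.
; Terminate and update events only forward to the parent, and the health check always reports healthy.
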(event `self.ProcessTerminate`
  (`parent.ProcessTerminate`))

(event `self.StartGameSession`
  (params (gameSession :type "AWSGameSessionServer Structure"))
  (`parent.StartGameSession` gameSession)
  (for _array_element (`.gameProperties` (break `AWSGameSessionServer` gameSession))
    (bind (_key _value) (break `GamePropertyServer` _array_element))
    (if (`KismetStringLibrary.EqualEqual_StrStr` _key "Game_Map")
      (`self.OnOpenLevel` (`KismetStringLibrary.Conv_StringToName` _value)))))

(event `self.UpdateGameSession`
  (params (updateGameSession :type "UpdateGameSessionServer Structure"))
  (`parent.UpdateGameSession` updateGameSession))

(fn `HealthCheck`
  (returns (ReturnValue :type Boolean))
  (return true))