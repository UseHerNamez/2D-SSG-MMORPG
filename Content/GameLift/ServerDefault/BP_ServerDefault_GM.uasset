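; Game mode for dedicated servers that registers the process with Amazon GameLift on BeginPlay.
; On a dedicated server it initializes the GameLift SDK, builds a BP_ProcessParams object with the server's port, and calls ProcessReady, printing the result.
; When the process params fire OnOpenLevel, it opens the requested level by name.
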(event `self.ReceiveBeginPlay`
  (if (`KismetSystemLibrary.IsDedicatedServer`)
    (bind _success (`GameLiftServerFunctionLibrary.InitSDK`))
    (if _success
      (bind _returnvalue (`|GenericCreateObject` "/Game/GameLift/BP_ProcessParams.BP_ProcessParams_C" self (`.port` (`ServerHelper.ServerIPAndPort`))))
      (add `/Game/GameLift/BP_ProcessParams.OnOpenLevel` _returnvalue (delegate `OnOpenLevel_Event_0`))
      (bind (_success_2 _errortype _errormessage) (`GameLiftServerFunctionLibrary.ProcessReady` _returnvalue))
      (if _success_2
        (`KismetSystemLibrary.PrintString` "init server gamelift sdk successfully!!")
        (else
          (`KismetSystemLibrary.PrintString` _errormessage))))))

(event `OnOpenLevel_Event_0`
  (params (Level :type Name))
  (`GameplayStatics.OpenLevel` Level))

(fn `UserConstructionScript`)