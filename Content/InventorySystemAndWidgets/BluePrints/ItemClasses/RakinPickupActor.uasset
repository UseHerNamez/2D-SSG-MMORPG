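; Pickup actor with a flipbook sprite that pops upward on spawn, falls under physics, then bobs once its vertical velocity reaches zero.
; Alternating component moves drive the bob until remaining lifespan runs low, when a timeline animates sprite alpha.
; ChasePlayerWhenPickedUp stops the bob and uses a timeline to pull the sprite to player 0's capsule while animating alpha, ignoring its PlayerREF input.
; SelfDestruct destroys the actor.
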(event `self.ReceiveBeginPlay`
  (bind _paperflipbook (`self.PaperFlipbook`))
  (bind _paperflipbook_2 (`self.PaperFlipbook`))
  (bind _paperflipbook_3 (`self.PaperFlipbook`))
  (bind _paperflipbook_4 (`self.PaperFlipbook`))
  (bind _returnvalue (`SceneComponent.K2_GetComponentLocation` _paperflipbook_2))
  (bind _returnvalue_2 (<= (`self.GetLifeSpan`) 1.2))
  (bind (_returnvalue_x _returnvalue_y _returnvalue_z) (`KismetMathLibrary.BreakVector` (`SceneComponent.GetComponentVelocity` _paperflipbook_4)))
  ;[1 1 1] Floating animation
  (`KismetSystemLibrary.Delay` 0.1)
  (`SceneComponent.K2_SetWorldLocation` _paperflipbook_3 (`SceneComponent.K2_GetComponentLocation` (`self.Sphere`)) false false)
  (`PrimitiveComponent.SetTranslucentSortPriority` _paperflipbook_3 10)
  (`PrimitiveComponent.SetTranslucentSortPriority` _paperflipbook_4 10)
  (`PrimitiveComponent.SetSimulatePhysics` _paperflipbook_4 true)
  (`PrimitiveComponent.SetPhysicsLinearVelocity` _paperflipbook_4 (0.0 0.0 200.0) true "None")
  (`PrimitiveComponent.SetEnableGravity` _paperflipbook_4 true)
  (if (== _returnvalue_z 0.0) :!label _label
    (`PrimitiveComponent.SetEnableGravity` _paperflipbook false)
    (`PrimitiveComponent.SetSimulatePhysics` _paperflipbook false)
    (`KismetSystemLibrary.MoveComponentTo` _paperflipbook_2 (+ _returnvalue (0.0 0.0 5.0)) (struct) true true 0.8 :!label _label_2)
    (`KismetSystemLibrary.Delay` 0.35 :!label _label_3)
    (if (`self.FloatingLoop`)
      (set `self.FloatingLoop` false)
      (if _returnvalue_2
        (bind (_direction _newtrack_0 _fade_away_gradually) (`Timeline|Timeline_1` :!label _label_4)
          (:`Update`
            (`PaperFlipbookComponent.SetSpriteColor` (`self.PaperFlipbook`) (make `LinearColor` 1.0 1.0 1.0 (`KismetMathLibrary.Lerp` 0.0 1.0 _fade_away_gradually)))))
        (else
          (`KismetSystemLibrary.MoveComponentTo` _paperflipbook_2 (- _returnvalue (0.0 0.0 5.0)) (struct) true true 0.8 :!label _label_5)
          (goto _label_3)))
      (else
        (set `self.FloatingLoop` true)
        (if _returnvalue_2
          (goto _label_4)
          (else
            (goto _label_2)))))
    (else
      (`KismetSystemLibrary.Delay` 0.15)
      (goto _label))))

(event `ChasePlayerWhenPickedUp`
  (params (playerREF :type "/Game/2DSideScrollerBP/Blueprints/2DSideScrollerCharacter Object Reference"))
  (bind _paperflipbook (`self.PaperFlipbook`))
  (`|ExecutionSequence`
    (:`then_0`
      (goto _label_2 :!via `Stop`))
    (:`then_1`
      (goto _label_5 :!via `Stop`))
    (:`then_2`
      (bind (_direction _fade_away_gradually _opacity) (`Timeline|Timeline_2` :!via `PlayFromStart`)
        (:`Update`
          (`SceneComponent.K2_SetWorldLocation` _paperflipbook (`KismetMathLibrary.VLerp` (`SceneComponent.K2_GetComponentLocation` (`self.PaperFlipbook`)) (`SceneComponent.K2_GetComponentLocation` (`Character.CapsuleComponent` (`GameplayStatics.GetPlayerCharacter` 0))) _opacity) false false)
          (`PaperFlipbookComponent.SetSpriteColor` _paperflipbook (make `LinearColor` 1.0 1.0 1.0 (`KismetMathLibrary.Lerp` 0.2 0.9 _fade_away_gradually))))))))

(event `SelfDestruct`
  (`self.K2_DestroyActor`))

(fn `UserConstructionScript`)