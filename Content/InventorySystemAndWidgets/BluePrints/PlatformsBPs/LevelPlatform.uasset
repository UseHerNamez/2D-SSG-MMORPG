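; LevelPlatform is a Paper2D platform that plays a repeating flipbook animation and is flagged as not jump-down-able.
; On BeginPlay it clears CanJumpDown, assigns its flipbook with looping off and enters an endless delay-driven cycle.
; Each cycle plays the animation, rewinds to the first frame, pauses, then randomizes the play rate to vary the next pass.
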(event `self.ReceiveBeginPlay`
  (bind _paperflipbook (`self.PaperFlipbook`))
  (set `self.CanJumpDown?` false)
  (`PaperFlipbookComponent.SetFlipbook` _paperflipbook "/Game/Sprites/Platforms/PlatformFB1.PlatformFB1")
  (`PaperFlipbookComponent.SetLooping` _paperflipbook false)
  (`PaperFlipbookComponent.PlayFromStart` _paperflipbook :!label _label)
  (`KismetSystemLibrary.Delay` 1.0)
  (`PaperFlipbookComponent.Stop` _paperflipbook)
  (`PaperFlipbookComponent.SetPlaybackPositionInFrames` _paperflipbook 0 false)
  (`KismetSystemLibrary.Delay` 1.0)
  (`PaperFlipbookComponent.SetPlayRate` _paperflipbook (`KismetMathLibrary.RandomFloatInRange` 1.0 1.8))
  (goto _label))

(fn `UserConstructionScript`)