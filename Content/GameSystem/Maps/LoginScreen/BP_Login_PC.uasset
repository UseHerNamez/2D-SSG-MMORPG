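; Login screen player controller, judging by its name, that animates the mouse cursor while the left button is held.
; A press starts a delay-driven loop through Hand, GrabHand and GrabHandClosed cursors, also reachable through a custom event.
; Release clears the held flag and restores the default cursor, so the loop stops at its next check.
; ShowErrorWidget is an empty event, and BeginPlay and Tick are disabled.
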(event `self.ShowErrorWidget`
  (params (ErrorMessage :type String)))

(event `change mouse cursor to click style`
  (set `self.CurrentMouseCursor` "Hand" :!label _label)
  (`KismetSystemLibrary.Delay` 0.2)
  (if (`self.leftClickDown?`)
    (set `self.CurrentMouseCursor` "GrabHand")
    (`KismetSystemLibrary.Delay` 0.2)
    (if (`self.leftClickDown?`)
      (set `self.CurrentMouseCursor` "GrabHandClosed")
      (`KismetSystemLibrary.Delay` 0.2)
      (if (`self.leftClickDown?`)
        (goto _label)))))

(event `Key|LeftMouseButton`
  (params (Key :type "Key Structure"))
  (:`Pressed`
    (set `self.leftClickDown?` true)
    (goto _label))
  (:`Released`
    (set `self.leftClickDown?` false)
    (set `self.CurrentMouseCursor` "Default")))

(fn `UserConstructionScript`)