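; Rakin pickup actor that pops upward on spawn, settles, then floats until it expires or is picked up.
; A polling loop makes the root and collision sphere follow the physics-driven flipbook, freezing it once it stops or starts rotating.
; Non-authority instances handle the bobbing, lifespan countdown with end-of-life fade, and fading chase toward the collecting player.
; Interface events trigger the chase and destruction, while functions expose collision bounds and item info.
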(event `self.ReceiveBeginPlay`
  (bind _paperflipbook (`self.PaperFlipbook`))
  (bind _paperflipbook_2 (`self.PaperFlipbook`))
  (bind _paperflipbook_3 (`self.PaperFlipbook`))
  (bind _paperflipbook_4 (`self.PaperFlipbook`))
  (bind _paperflipbook_5 (`self.PaperFlipbook`))
  (bind _returnvalue (`SceneComponent.K2_GetComponentLocation` _paperflipbook_2))
  (bind _returnvalue_2 (<= (`self.LifeSpan`) 2.0))
  ;[1 1 1] Floating animation
  (`self.EventSetClientLifeSpan` (`self.GetLifeSpan`))
  (`KismetSystemLibrary.Delay` 0.1)
  (`SceneComponent.K2_SetWorldLocation` _paperflipbook_3 (`SceneComponent.K2_GetComponentLocation` (`self.Sphere`)) false false)
  (`PrimitiveComponent.SetTranslucentSortPriority` _paperflipbook_3 25)
  (`PrimitiveComponent.SetSimulatePhysics` _paperflipbook_4 true)
  (`PrimitiveComponent.SetPhysicsLinearVelocity` _paperflipbook_4 (0.0 0.0 400.0) true "None")
  (`PrimitiveComponent.SetEnableGravity` _paperflipbook_4 true)
  (if (not (`KismetMathLibrary.EqualExactly_VectorVector` (`SceneComponent.GetComponentVelocity` _paperflipbook_4))) :!label _label
    (`SceneComponent.K2_SetWorldLocation` (`self.Sphere`) (`SceneComponent.K2_GetComponentLocation` (`self.PaperFlipbook`)) false true)
    (`SceneComponent.K2_SetWorldLocation` (`self.Scene`) (`SceneComponent.K2_GetComponentLocation` (`self.PaperFlipbook`)) false true)
    (if (!= (`SceneComponent.K2_GetComponentRotation` _paperflipbook_4) (struct) :`ErrorTolerance` 0.0)
      (`SceneComponent.K2_SetWorldRotation` :`self` _paperflipbook_4 :`bTeleport` true)
      (else
        (`KismetSystemLibrary.Delay` 0.15)
        (goto _label))))
  (`PrimitiveComponent.SetEnableGravity` _paperflipbook false)
  (`PrimitiveComponent.SetSimulatePhysics` _paperflipbook false)
  (`SceneComponent.K2_SetWorldLocation` (`self.Scene`) _returnvalue false true)
  (`SceneComponent.K2_SetWorldLocation` (`self.Sphere`) _returnvalue false true)
  (`SceneComponent.K2_SetWorldLocation` _paperflipbook_2 _returnvalue false true)
  (`/Engine/EditorBlueprintResources/ActorMacros.Switch Has Authority`
    (:`Remote`
      (`KismetSystemLibrary.MoveComponentTo` _paperflipbook_2 (+ _returnvalue (0.0 0.0 5.0)) (struct) true true 0.8 :!label _label_2)
      (`KismetSystemLibrary.Delay` 0.35 :!label _label_3)
      (if (`self.FloatingLoop`)
        (set `self.FloatingLoop` false)
        (if _returnvalue_2
          _
          (else
            (`KismetSystemLibrary.MoveComponentTo` _paperflipbook_2 (- _returnvalue (0.0 0.0 5.0)) (struct) true true 0.8 :!label _label_4)
            (goto _label_3)))
        (else
          (set `self.FloatingLoop` true)
          (if _returnvalue_2
            _
            (else
              (goto _label_2)))))
      (`PaperFlipbookComponent.Stop` _paperflipbook_5)
      (bind (_direction _newtrack_0 _fade_away_gradually) (`Timeline|Timeline_1`)
        (:`Update`
          (`PaperFlipbookComponent.SetSpriteColor` _paperflipbook_5 (make `LinearColor` 1.0 1.0 1.0 (`KismetMathLibrary.Lerp` 0.0 1.0 _fade_away_gradually))))))))

(event `EventSetClientLifeSpan`
  (params (LifeSpan :type "Float (double-precision)"))
  (`/Engine/EditorBlueprintResources/ActorMacros.Switch Has Authority`
    (:`Remote`
      (set `self.LifeSpan` LifeSpan)
      (bind _returnvalue (`KismetSystemLibrary.K2_SetTimerDelegate` (delegate `TimerEventSetClientLifeSpan`) 1.0 true))
      (set `self.LifeSpanTimeHandler` _returnvalue))))

(event `TimerEventSetClientLifeSpan`
  (set `self.LifeSpan` (- (`self.LifeSpan`) 1.0)))

(event `ChasePlayerWhenPickedUp`
  (params (playerREF :type "PaperCharacter Object Reference (by ref)"))
  (bind _paperflipbook (`self.PaperFlipbook`))
  (`/Engine/EditorBlueprintResources/ActorMacros.Switch Has Authority`
    (:`Remote`
      (`|ExecutionSequence`
        (:`then_0`
          (goto _label_2 :!via `Stop`))
        (:`then_1`
          (goto _label_4 :!via `Stop`))
        (:`then_2`
          (bind (_direction _fade_away_gradually _opacity) (`Timeline|Timeline_2` :!via `PlayFromStart`)
            (:`Update`
              (`SceneComponent.K2_SetWorldLocation` _paperflipbook (`KismetMathLibrary.VLerp` (`SceneComponent.K2_GetComponentLocation` (`self.PaperFlipbook`)) (`SceneComponent.K2_GetComponentLocation` (`Character.CapsuleComponent` playerREF)) _opacity) false false)
              (`PaperFlipbookComponent.SetSpriteColor` _paperflipbook (make `LinearColor` 1.0 1.0 1.0 (`KismetMathLibrary.Lerp` 0.2 0.9 _fade_away_gradually))))))))))

(event `/Game/GameSystem/BluePrints/BPInterface_PickupObjects.Chase player interface`
  (params (`Char ref` :type "Character Object Reference"))
  (`self.ChasePlayerWhenPickedUp` `Char ref`))

(event `SelfDestruct`
  (`self.K2_DestroyActor`))

(event `/Game/GameSystem/BluePrints/BPInterface_PickupObjects.self destruct interface`
  (`self.SelfDestruct`))

(fn `return collision bounds`
  (returns (`Sphere REF` :type "SphereComponent Object Reference"))
  (return (`self.Sphere`)))

(fn `return item info`
  (returns (`item info` :type "/Game/GameSystem/Structures/S_PickupItemInfo Structure") (`rakin info` :type "/Game/GameSystem/Structures/Rakins_Struct Structure"))
  (return (struct) (`self.rakins`)))

(fn `UserConstructionScript`)