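; Game instance Blueprint that holds portal state and saved character stats and level, exposed through getter functions.
; The BPISearchGameSession event is currently empty.
; Disconnected logic would query an AWS GameLift alias for sessions matching a map property, travel to the first result's IP and port, then clear the RightPortal flag.
; DisplayErrorMsg is an empty stub.
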(event `/Game/GameSystem/BluePrints/BPI_GameInstance.BPISearchGameSession`
  (params (LevelToSearch :type Name))
  ;[1 1 1] Search gameplay server map
)

(fn `get portal bool var`
  (returns (`right portal?` :type Boolean))
  (return (`self.right Portal?`)))

(fn `get saved vars`
  (returns (`saved?` :type Boolean) (stats :type "/Game/GameSystem/Structures/S_RepCharStatsModifiersVars Structure") (lvl :type Integer))
  (return (`self.existing load?`) (`self.char stats`) (`self.char lvl`)))