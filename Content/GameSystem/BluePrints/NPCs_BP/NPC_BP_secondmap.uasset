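; NPC Blueprint for the second map that sets itself up as the quest NPC "AVAlphaUnit", inheriting the rest from its parent.
; On BeginPlay it uses that name as the row key into the AllQuestsInfos_DT data table, loading its quests and quest-widget sprite.
; When the row is found, the authority instance then registers itself by name in the 2DGameStateBase NPC reference list.
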(event `self.ReceiveBeginPlay`
  (`parent.ReceiveBeginPlay`)
  (bind _output_get (set `self.NPC_name` "AVAlphaUnit"))
  (bind _returnvalue (`|GetDataTableRow` "/Game/GameSystem/DataTables/AllQuestsInfos_DT.AllQuestsInfos_DT" _output_get)
    (:`then`
      (bind (_npcname _npcsprite _allquestsinfo) (break `/Game/GameSystem/Structures/S_QuestNPC_Info` _returnvalue))
      (set `self.Quests` _allquestsinfo)
      (set `self.sprite for quest widgets` _npcsprite)
      (`/Engine/EditorBlueprintResources/ActorMacros.Switch Has Authority`
        (:`Authority`
          (bind _as2dgame_state_base (cast `/Game/2DSideScrollerBP/Blueprints/2DGameStateBase` (`GameplayStatics.GetGameState`)))
          (`/Game/2DSideScrollerBP/Blueprints/2DGameStateBase.AddToNpcRefArr_Serv` _as2dgame_state_base self (`self.NPC_name`)))))))

(fn `UserConstructionScript`
  (`parent.UserConstructionScript`))