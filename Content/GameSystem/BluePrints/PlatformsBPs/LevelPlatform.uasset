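; A level platform for the 2D side-scroller with an animated flipbook and a Box trigger that can end the character's flying movement.
; From BeginPlay, a delay loop repeatedly plays the flipbook, rewinds it to the first frame, pauses, and re-randomizes its play rate.
; When a 2DSideScrollerCharacter begins overlapping the Box while holding Down in Flying mode, its movement switches to Walking.
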(event `self.ReceiveBeginPlay`
  (bind _paperflipbook (`self.PaperFlipbook`))
  (set `self.CanJumpDown?` false)
  (`PaperFlipbookComponent.SetFlipbook` _paperflipbook "/Game/GameSystem/Textures/Platforms/WhereTheJourneyBegins/OtherPlatforms/PlatformFB1.PlatformFB1")
  (`PaperFlipbookComponent.SetLooping` _paperflipbook false)
  (`PaperFlipbookComponent.PlayFromStart` _paperflipbook :!label _label)
  (`KismetSystemLibrary.Delay` 1.0)
  (`PaperFlipbookComponent.Stop` _paperflipbook)
  (`PaperFlipbookComponent.SetPlaybackPositionInFrames` _paperflipbook 0 false)
  (`KismetSystemLibrary.Delay` 1.0)
  (`PaperFlipbookComponent.SetPlayRate` _paperflipbook (`KismetMathLibrary.RandomFloatInRange` 1.0 1.8))
  (goto _label))

(event `self.Box.OnComponentBeginOverlap`
  (params (OverlappedComponent :type "PrimitiveComponent Object Reference") (OtherActor :type "Actor Object Reference") (OtherComp :type "PrimitiveComponent Object Reference") (OtherBodyIndex :type Integer) (bFromSweep :type Boolean) (SweepResult :type "HitResult Structure (by ref)"))
  (bind _as2dside_scroller_character (cast `/Game/2DSideScrollerBP/Blueprints/2DSideScrollerCharacter` OtherActor))
  (bind _charactermovement (`Character.CharacterMovement` _as2dside_scroller_character))
  (if (and (`/Game/2DSideScrollerBP/Blueprints/2DSideScrollerCharacter.downKeyPressed` _as2dside_scroller_character) (`|EnumEquality` (`CharacterMovementComponent.MovementMode` _charactermovement) "MOVE_Flying"))
    (`CharacterMovementComponent.SetMovementMode` _charactermovement "MOVE_Walking" 0)))

(fn `UserConstructionScript`)