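; One-way floating platform that the 2D side-scroller character can pass through from below or drop down through from above.
; The UnderCollision volume turns Platform collision off on overlap and back on when the character leaves it.
; The Above volume, also checked shortly after BeginPlay, enables input and opens a Gate that lets Down plus Jump, or held Down+Alt, disable collision.
; Leaving Above disables input and closes the Gate.
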(event `self.UnderCollision.OnComponentBeginOverlap`
  (params (OverlappedComponent :type "PrimitiveComponent Object Reference") (OtherActor :type "Actor Object Reference") (OtherComp :type "PrimitiveComponent Object Reference") (OtherBodyIndex :type Integer) (bFromSweep :type Boolean) (SweepResult :type "HitResult Structure (by ref)"))
  (cast `/Game/2DSideScrollerBP/Blueprints/2DSideScrollerCharacter` OtherActor)
  (`PrimitiveComponent.SetCollisionEnabled` (`self.Platform`) "NoCollision"))

(event `self.UnderCollision.OnComponentEndOverlap`
  (params (OverlappedComponent :type "PrimitiveComponent Object Reference") (OtherActor :type "Actor Object Reference") (OtherComp :type "PrimitiveComponent Object Reference") (OtherBodyIndex :type Integer))
  (bind _as2dside_scroller_character (cast `/Game/2DSideScrollerBP/Blueprints/2DSideScrollerCharacter` OtherActor))
  (`PrimitiveComponent.SetCollisionEnabled` (`self.Platform`) "QueryAndPhysics"))

(event `self.ReceiveBeginPlay`
  (set `self.CanJumpDown?` true)
  (`KismetSystemLibrary.Delay` 0.1)
  (if (`PrimitiveComponent.IsOverlappingActor` (`self.Above`) (`GameplayStatics.GetPlayerCharacter` 0))
    (`self.EnableInput` (`GameplayStatics.GetPlayerController` 0) :!label _label)
    (goto _label_2 :!via `Open`)))

(event `self.Above.OnComponentBeginOverlap`
  (params (OverlappedComponent :type "PrimitiveComponent Object Reference") (OtherActor :type "Actor Object Reference") (OtherComp :type "PrimitiveComponent Object Reference") (OtherBodyIndex :type Integer) (bFromSweep :type Boolean) (SweepResult :type "HitResult Structure (by ref)"))
  (bind _returnvalue (`GameplayStatics.GetPlayerController` 0))
  (cast `/Game/2DSideScrollerBP/Blueprints/2DSideScrollerCharacter` OtherActor)
  (`|ExecutionSequence`
    (:`then_0`
      (goto _label))
    (:`then_1`
      (`KismetSystemLibrary.Delay` 0.3)
      (if (and (`PlayerController.IsInputKeyDown` _returnvalue "Down") (or (`PlayerController.IsInputKeyDown` _returnvalue "LeftAlt") (`PlayerController.IsInputKeyDown` _returnvalue "RightAlt")))
        (`/Engine/EditorBlueprintResources/StandardMacros.Gate` true :!label _label_2
          (:`Exit`
            (`PrimitiveComponent.SetCollisionEnabled` (`self.Platform`) "NoCollision")))))))

(event `InputAction|Jump` :consume false
  (params (Key :type "Key Structure"))
  (:`Pressed`
    (if (`PlayerController.IsInputKeyDown` (`GameplayStatics.GetPlayerController` 0) "Down")
      (goto _label_2))))

(event `self.Above.OnComponentEndOverlap`
  (params (OverlappedComponent :type "PrimitiveComponent Object Reference") (OtherActor :type "Actor Object Reference") (OtherComp :type "PrimitiveComponent Object Reference") (OtherBodyIndex :type Integer))
  (cast `/Game/2DSideScrollerBP/Blueprints/2DSideScrollerCharacter` OtherActor)
  (`self.DisableInput` (`GameplayStatics.GetPlayerController` 0))
  (goto _label_2 :!via `Close`))

(fn `UserConstructionScript`)