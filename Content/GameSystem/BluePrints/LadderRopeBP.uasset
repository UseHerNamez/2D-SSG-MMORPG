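; Climbable ladder or rope for the 2D side-scroller character, usable from below or from the top.
; Overlaps on the climb and top boxes, plus two callable functions, check Up/Down input to set Flying mode, X plane constraint and horizontal snapping.
; Overlapping FloatPlatforms are ignored for collision so the character passes through, with most snapping gated on finding one.
; Leaving the volumes clears climbing, restoring Falling and default constraints, with a lift at the top.
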(event `self.ClimbCollision.OnComponentBeginOverlap`
  (params (OverlappedComponent :type "PrimitiveComponent Object Reference") (OtherActor :type "Actor Object Reference") (OtherComp :type "PrimitiveComponent Object Reference") (OtherBodyIndex :type Integer) (bFromSweep :type Boolean) (SweepResult :type "HitResult Structure (by ref)"))
  (bind _returnvalue_x (`KismetMathLibrary.BreakVector` (`SceneComponent.K2_GetComponentLocation` (`self.ClimbCollision`))))
  (bind _output (`|GetArrayItem` (`PrimitiveComponent.GetOverlappingActors` (`self.Ladder or Rope`) "/Game/GameSystem/BluePrints/PlatformsBPs/FloatPlatform.FloatPlatform_C")))
  (bind _as2dside_scroller_character (cast `/Game/2DSideScrollerBP/Blueprints/2DSideScrollerCharacter` OtherActor))
  (if (`/Game/2DSideScrollerBP/Blueprints/2DSideScrollerCharacter.upKeyPressed` _as2dside_scroller_character)
    (set `/Game/2DSideScrollerBP/Blueprints/2DSideScrollerCharacter.climbingRope` true _as2dside_scroller_character)
    (if (`KismetSystemLibrary.IsValid` _output)
      (bind _asfloat_platform (cast `/Game/GameSystem/BluePrints/PlatformsBPs/FloatPlatform` _output))
      (`/Game/2DSideScrollerBP/Blueprints/2DSideScrollerCharacter.ChangeIgnoreActors` _as2dside_scroller_character (`/Game/GameSystem/BluePrints/PlatformsBPs/MasterPlatform.Platform` _asfloat_platform) true)
      (bind _charactermovement (`Character.CharacterMovement` _as2dside_scroller_character))
      (`CharacterMovementComponent.SetMovementMode` _charactermovement "MOVE_Flying" 0)
      (`MovementComponent.StopMovementImmediately` _charactermovement)
      (`MovementComponent.SetPlaneConstraintAxisSetting` _charactermovement "X")
      (bind (_returnvalue_x_2 _returnvalue_y _returnvalue_z) (`KismetMathLibrary.BreakVector` (`SceneComponent.K2_GetComponentLocation` (`Actor.RootComponent` _as2dside_scroller_character))))
      (`SceneComponent.K2_SetWorldLocation` (`Character.CapsuleComponent` _as2dside_scroller_character) (`KismetMathLibrary.MakeVector` _returnvalue_x 0.0 _returnvalue_z) false false)
      (`SceneComponent.K2_SetWorldLocation` (`Actor.RootComponent` _as2dside_scroller_character) (`KismetMathLibrary.MakeVector` _returnvalue_x 0.0 _returnvalue_z) false false))))

(event `self.ClimbCollision.OnComponentEndOverlap`
  (params (OverlappedComponent :type "PrimitiveComponent Object Reference") (OtherActor :type "Actor Object Reference") (OtherComp :type "PrimitiveComponent Object Reference") (OtherBodyIndex :type Integer))
  (bind _as2dside_scroller_character (cast `/Game/2DSideScrollerBP/Blueprints/2DSideScrollerCharacter` OtherActor))
  (if (!= (`KismetArrayLibrary.Array_Find` (`self.GetOverlappingComponents` _as2dside_scroller_character) (`self.TopLadderCollisionBox`)) -1)
    (bind _rootcomponent (`Actor.RootComponent` _as2dside_scroller_character))
    (bind (_returnvalue_x _returnvalue_y _returnvalue_z) (`KismetMathLibrary.BreakVector` (`SceneComponent.K2_GetComponentLocation` _rootcomponent)))
    (`SceneComponent.K2_SetWorldLocation` _rootcomponent (`KismetMathLibrary.MakeVector` _returnvalue_x 0.0 (+ _returnvalue_z 10.0)) false false)
    (set `/Game/2DSideScrollerBP/Blueprints/2DSideScrollerCharacter.climbingRope` false _as2dside_scroller_character :!label _label)
    (bind _charactermovement (`Character.CharacterMovement` _as2dside_scroller_character))
    (if (not (`|EnumEquality` (`CharacterMovementComponent.MovementMode` _charactermovement) "MOVE_Walking"))
      (`CharacterMovementComponent.SetMovementMode` _charactermovement "MOVE_Falling" 0)
      (`MovementComponent.SetPlaneConstraintAxisSetting` _charactermovement "UseGlobalPhysicsSetting"))
    (elif (not (`PrimitiveComponent.IsOverlappingActor` (`self.Ladder or Rope`) _as2dside_scroller_character))
      (goto _label))))

(event `self.TopLadderCollisionBox.OnComponentBeginOverlap`
  (params (OverlappedComponent :type "PrimitiveComponent Object Reference") (OtherActor :type "Actor Object Reference") (OtherComp :type "PrimitiveComponent Object Reference") (OtherBodyIndex :type Integer) (bFromSweep :type Boolean) (SweepResult :type "HitResult Structure (by ref)"))
  (bind _returnvalue_x (`KismetMathLibrary.BreakVector` (`SceneComponent.K2_GetComponentLocation` (`self.TopLadderCollisionBox`))))
  (bind _output (`|GetArrayItem` (`PrimitiveComponent.GetOverlappingActors` (`self.Ladder or Rope`) "/Game/GameSystem/BluePrints/PlatformsBPs/FloatPlatform.FloatPlatform_C")))
  (bind _as2dside_scroller_character (cast `/Game/2DSideScrollerBP/Blueprints/2DSideScrollerCharacter` OtherActor))
  (if (`/Game/2DSideScrollerBP/Blueprints/2DSideScrollerCharacter.downKeyPressed` _as2dside_scroller_character)
    (set `/Game/2DSideScrollerBP/Blueprints/2DSideScrollerCharacter.climbingRope` true _as2dside_scroller_character)
    (if (`KismetSystemLibrary.IsValid` _output)
      (bind _asfloat_platform (cast `/Game/GameSystem/BluePrints/PlatformsBPs/FloatPlatform` _output))
      (`/Game/2DSideScrollerBP/Blueprints/2DSideScrollerCharacter.ChangeIgnoreActors` _as2dside_scroller_character (`/Game/GameSystem/BluePrints/PlatformsBPs/MasterPlatform.Platform` _asfloat_platform) true)
      (bind _charactermovement (`Character.CharacterMovement` _as2dside_scroller_character))
      (`CharacterMovementComponent.SetMovementMode` _charactermovement "MOVE_Flying" 0)
      (`MovementComponent.SetPlaneConstraintAxisSetting` _charactermovement "X")
      (bind _rootcomponent (`Actor.RootComponent` _as2dside_scroller_character))
      (bind (_returnvalue_x_2 _returnvalue_y _returnvalue_z) (`KismetMathLibrary.BreakVector` (`SceneComponent.K2_GetComponentLocation` _rootcomponent)))
      (`SceneComponent.K2_SetWorldLocation` _rootcomponent (`KismetMathLibrary.MakeVector` _returnvalue_x 0.0 (- _returnvalue_z 10.0)) false false))))

(event `self.TopLadderCollisionBox.OnComponentEndOverlap`
  (params (OverlappedComponent :type "PrimitiveComponent Object Reference") (OtherActor :type "Actor Object Reference") (OtherComp :type "PrimitiveComponent Object Reference") (OtherBodyIndex :type Integer))
  (bind _as2dside_scroller_character (cast `/Game/2DSideScrollerBP/Blueprints/2DSideScrollerCharacter` OtherActor))
  (`PrimitiveComponent.SetCollisionEnabled` (`Character.CapsuleComponent` _as2dside_scroller_character) "QueryAndPhysics")
  (if (not (!= (`KismetArrayLibrary.Array_Find` (`self.GetOverlappingComponents` _as2dside_scroller_character) (`self.ClimbCollision`)) -1))
    (bind _charactermovement (`Character.CharacterMovement` _as2dside_scroller_character))
    (bind _movementmode (`CharacterMovementComponent.MovementMode` _charactermovement))
    (if (not (or (`|EnumEquality` _movementmode "MOVE_Walking") (`|EnumEquality` _movementmode "MOVE_Falling")))
      (`CharacterMovementComponent.SetMovementMode` _charactermovement "MOVE_Falling" 0))
    (set `/Game/2DSideScrollerBP/Blueprints/2DSideScrollerCharacter.climbingRope` false _as2dside_scroller_character)
    (`MovementComponent.SetPlaneConstraintAxisSetting` _charactermovement "UseGlobalPhysicsSetting")))

(event `self.Ladder or Rope.OnComponentBeginOverlap`
  (params (OverlappedComponent :type "PrimitiveComponent Object Reference") (OtherActor :type "Actor Object Reference") (OtherComp :type "PrimitiveComponent Object Reference") (OtherBodyIndex :type Integer) (bFromSweep :type Boolean) (SweepResult :type "HitResult Structure (by ref)"))
  (bind _output (`|GetArrayItem` (`PrimitiveComponent.GetOverlappingActors` (`self.Ladder or Rope`) "/Game/GameSystem/BluePrints/PlatformsBPs/FloatPlatform.FloatPlatform_C")))
  (bind _as2dside_scroller_character (cast `/Game/2DSideScrollerBP/Blueprints/2DSideScrollerCharacter` OtherActor))
  (if (`KismetSystemLibrary.IsValid` _output)
    (bind _asfloat_platform (cast `/Game/GameSystem/BluePrints/PlatformsBPs/FloatPlatform` _output))
    (`/Game/2DSideScrollerBP/Blueprints/2DSideScrollerCharacter.ChangeIgnoreActors` _as2dside_scroller_character (`/Game/GameSystem/BluePrints/PlatformsBPs/MasterPlatform.Platform` _asfloat_platform) true)))

(fn `ChangeToClimbModeDown`
  (params (Char :type "/Game/2DSideScrollerBP/Blueprints/2DSideScrollerCharacter Object Reference"))
  (bind _charactermovement (`Character.CharacterMovement` Char))
  (bind _capsulecomponent (`Character.CapsuleComponent` Char))
  (bind _returnvalue_x (`KismetMathLibrary.BreakVector` (`SceneComponent.K2_GetComponentLocation` (`self.TopLadderCollisionBox`))))
  (bind (_returnvalue_x_2 _returnvalue_y _returnvalue_z) (`KismetMathLibrary.BreakVector` (`SceneComponent.K2_GetComponentLocation` _capsulecomponent)))
  (bind _output (`|GetArrayItem` (`self.GetOverlappingActors` Char "/Game/GameSystem/BluePrints/PlatformsBPs/FloatPlatform.FloatPlatform_C")))
  (if (!= (`KismetArrayLibrary.Array_Find` (`PrimitiveComponent.GetOverlappingActors` (`self.TopLadderCollisionBox`) "/Game/2DSideScrollerBP/Blueprints/2DSideScrollerCharacter.2DSideScrollerCharacter_C") Char) -1)
    (if (`/Game/2DSideScrollerBP/Blueprints/2DSideScrollerCharacter.downKeyPressed` Char)
      (`CharacterMovementComponent.SetMovementMode` _charactermovement "MOVE_Flying" 0)
      (set `/Game/2DSideScrollerBP/Blueprints/2DSideScrollerCharacter.climbingRope` true Char)
      (if (`KismetSystemLibrary.IsValid` _output)
        (bind _asfloat_platform (cast `/Game/GameSystem/BluePrints/PlatformsBPs/FloatPlatform` _output))
        (`PrimitiveComponent.IgnoreComponentWhenMoving` _capsulecomponent (`/Game/GameSystem/BluePrints/PlatformsBPs/MasterPlatform.Platform` _asfloat_platform) true)
        (`MovementComponent.SetPlaneConstraintAxisSetting` _charactermovement "X")
        (`SceneComponent.K2_SetWorldLocation` _capsulecomponent (`KismetMathLibrary.MakeVector` _returnvalue_x 0.0 (- _returnvalue_z 10.0)) false false)
        (return))
      (else
        (return)))
    (else
      (return))))

(fn `ChangeToClimbModeUp`
  (params (Character :type "/Game/2DSideScrollerBP/Blueprints/2DSideScrollerCharacter Object Reference"))
  (bind _charactermovement (`Character.CharacterMovement` Character))
  (bind _capsulecomponent (`Character.CapsuleComponent` Character))
  (bind _returnvalue_x (`KismetMathLibrary.BreakVector` (`SceneComponent.K2_GetComponentLocation` (`self.ClimbCollision`))))
  (bind (_returnvalue_x_2 _returnvalue_y _returnvalue_z) (`KismetMathLibrary.BreakVector` (`SceneComponent.K2_GetComponentLocation` _capsulecomponent)))
  (bind _output (`|GetArrayItem` (`PrimitiveComponent.GetOverlappingActors` (`self.Ladder or Rope`) "/Game/GameSystem/BluePrints/PlatformsBPs/FloatPlatform.FloatPlatform_C")))
  (if (!= (`KismetArrayLibrary.Array_Find` (`PrimitiveComponent.GetOverlappingActors` (`self.ClimbCollision`) "/Game/2DSideScrollerBP/Blueprints/2DSideScrollerCharacter.2DSideScrollerCharacter_C") Character) -1)
    (if (`/Game/2DSideScrollerBP/Blueprints/2DSideScrollerCharacter.upKeyPressed` Character)
      (`CharacterMovementComponent.SetMovementMode` _charactermovement "MOVE_Flying" 0)
      (set `/Game/2DSideScrollerBP/Blueprints/2DSideScrollerCharacter.climbingRope` true Character)
      (if (`KismetSystemLibrary.IsValid` _output)
        (bind _asfloat_platform (cast `/Game/GameSystem/BluePrints/PlatformsBPs/FloatPlatform` _output)
          (:`then`
            (`/Game/2DSideScrollerBP/Blueprints/2DSideScrollerCharacter.ChangeIgnoreActors` Character (`/Game/GameSystem/BluePrints/PlatformsBPs/MasterPlatform.Platform` _asfloat_platform) true))
          (:`CastFailed`
            _))
        (`MovementComponent.StopMovementImmediately` _charactermovement)
        (`MovementComponent.SetPlaneConstraintAxisSetting` _charactermovement "X")
        (`SceneComponent.K2_SetWorldLocation` _capsulecomponent (`KismetMathLibrary.MakeVector` _returnvalue_x 0.0 _returnvalue_z) false false)
        (return))
      (else
        (return)))
    (else
      (return))))

(fn `UserConstructionScript`)