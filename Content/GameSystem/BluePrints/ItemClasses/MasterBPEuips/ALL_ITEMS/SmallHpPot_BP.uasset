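; Small health potion item that restores a fixed amount of HP to the inventory's owning character when used.
; On use, if current HP is below max, it applies the usable effect and removes one from a fixed inventory array, ignoring the passed-in array argument.
; It then destroys its actor after a short delay; at full HP it destroys the actor immediately without consuming the item.
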(event `EventOnUsed_1`
  (params (`Which Array` :type "/Game/GameSystem/BluePrints/Enums/E_ItemCategories Enum" :default "NewEnumerator0"))
  (bind _charref (`/Game/GameSystem/BluePrints/BP_Inventory.CharRef` (`self.Inventory`)))
  (bind (_stats_struct_var_charmaxhp _stats_struct_var_charcurrhp) (break `/Game/GameSystem/BluePrints/Structures/CharactersStats_Struct` (`/Game/2DSideScrollerBP/Blueprints/2DSideScrollerCharacter.Stats_struct var` _charref)))
  (if (< _stats_struct_var_charcurrhp _stats_struct_var_charmaxhp)
    (`/Game/2DSideScrollerBP/Blueprints/2DSideScrollerCharacter.Apply Useable Effect` :`self` _charref :`Amount` 10)
    (`/Game/GameSystem/BluePrints/BP_Inventory.RemoveItemAtIndex` (`self.Inventory`) (`self.Index`) 1 "NewEnumerator1")
    (`KismetSystemLibrary.Delay` 0.05)
    (`self.K2_DestroyActor`)
    (else
      (`self.K2_DestroyActor`))))

(fn `UserConstructionScript`
  (`parent.UserConstructionScript`))