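; World pickup actor that shows an item's sprite and animates its drop, idle float and collection.
; BeginPlay launches the sprite upward and polls until physics velocity is zero, then disables physics and starts a looping eased bob.
; The bob loop switches to a timeline alpha fade when lifespan nears its end.
; A pickup event stops the bob and lerps the sprite toward player 0 while fading, with a separate event destroying the actor.
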(event `self.ReceiveBeginPlay`
  (bind _icon_sprite (`self.Icon_Sprite`))
  (bind _icon_sprite_2 (`self.Icon_Sprite`))
  (bind _scene (`self.Scene`))
  (bind _returnvalue (<= (`self.GetLifeSpan`) 1.2))
  (bind _returnvalue_2 (`SceneComponent.K2_GetComponentLocation` _icon_sprite_2))
  (bind (_returnvalue_x _returnvalue_y _returnvalue_z) (`KismetMathLibrary.BreakVector` (`SceneComponent.GetComponentVelocity` (`self.Icon_Sprite`))))
  ;[1 1 1] Floating animation
  (`self.SetReplicateMovement` self false)
  (`PaperSpriteComponent.SetSprite` (`self.Icon_Sprite`) (`.SpriteOfTheTexture_51_26F6AB1D48E0EBC0D119538F6944E051` (break `/Game/GameSystem/Structures/Struct_ItemProperties` (`.ItemPropertiesStruct_14_60179F8943E4075BC3DE8680B21848D6` (break `/Game/GameSystem/Structures/S_PickupItemInfo` (`self.ItemInformation`))))))
  (`PrimitiveComponent.SetPhysicsLinearVelocity` (`self.Icon_Sprite`) (0.0 0.0 500.0) true "None")
  (if (and (== _returnvalue_x 0.0) (== _returnvalue_y 0.0) (== _returnvalue_z 0.0)) :!label _label
    (`PrimitiveComponent.SetEnableGravity` _icon_sprite_2 false)
    (`PrimitiveComponent.SetSimulatePhysics` _icon_sprite false)
    (`KismetSystemLibrary.MoveComponentTo` _icon_sprite_2 (+ _returnvalue_2 (0.0 0.0 5.0)) (struct) false false 0.8)
    (`SceneComponent.K2_SetWorldLocation` _scene _returnvalue_2 false false)
    (`KismetSystemLibrary.MoveComponentTo` _icon_sprite (+ (`SceneComponent.K2_GetComponentLocation` _scene) (0.0 0.0 5.0)) (struct) true true 0.8 :!label _label_2)
    (`KismetSystemLibrary.Delay` 0.6 :!label _label_3)
    (if (`self.FloatingLoop`)
      (set `self.FloatingLoop` false)
      (if _returnvalue
        (bind (_direction _newtrack_0 _fade_away_gradually) (`Timeline|Timeline_1` :!label _label_4)
          (:`Update`
            (`PaperSpriteComponent.SetSpriteColor` (`self.Icon_Sprite`) (make `LinearColor` 1.0 1.0 1.0 (`KismetMathLibrary.Lerp` 0.0 1.0 _fade_away_gradually)))))
        (else
          (`KismetSystemLibrary.MoveComponentTo` _icon_sprite (- _returnvalue_2 (0.0 0.0 5.0)) (struct) true true 0.8 :!label _label_5)
          (goto _label_3)))
      (else
        (set `self.FloatingLoop` true)
        (if _returnvalue
          (goto _label_4)
          (else
            (goto _label_2)))))
    (else
      (`KismetSystemLibrary.Delay` 0.1)
      (goto _label))))

(event `ChasePalyerWhenrPickup`
  (`|ExecutionSequence`
    (:`then_0`
      (goto _label_2 :!via `Stop`))
    (:`then_1`
      (goto _label_5 :!via `Stop`))
    (:`then_2`
      (bind (_direction _fade_away_gradually _opacity) (`Timeline|Timeline_2` :!via `PlayFromStart`)
        (:`Update`
          (`SceneComponent.K2_SetWorldLocation` (`self.Icon_Sprite`) (`KismetMathLibrary.VLerp` (`SceneComponent.K2_GetComponentLocation` (`self.Icon_Sprite`)) (`SceneComponent.K2_GetComponentLocation` (`Character.CapsuleComponent` (`GameplayStatics.GetPlayerCharacter` 0))) _opacity) false false)
          (`PaperSpriteComponent.SetSpriteColor` (`self.Icon_Sprite`) (make `LinearColor` 1.0 1.0 1.0 (`KismetMathLibrary.Lerp` 0.1 1.0 _fade_away_gradually))))))))

(event `SelfDestruct`
  (`self.K2_DestroyActor`))

(fn `UserConstructionScript`)