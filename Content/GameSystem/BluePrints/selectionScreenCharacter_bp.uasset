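; Paper2D character preview for the selection screen that layers equipment, face and hair sprites onto flipbook sockets.
; AddEquip parses slot:item strings to pick a data table, or on finishing adds face and hair (none under a hat), or just the part named by CreationStr.
; Draw order comes from the Idle/Alert translucency priority row.
; getCorrectTextureStyle indexes composite tables' parent tables by gender and style, then rows by color.
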(event `self.ReceiveBeginPlay`
  (bind _paperflipbook (`self.PaperFlipbook`))
  (`PrimitiveComponent.SetTranslucentSortPriority` _paperflipbook 13)
  (bind _output_get (set `self.charFB` (`PaperFlipbookComponent.GetFlipbook` _paperflipbook)))
  (`/Engine/EditorBlueprintResources/StandardMacros.IsValid` _output_get
    (:`Is Valid`
      (`KismetSystemLibrary.PrintString` "valid in bp"))
    (:`Is Not Valid`
      (`KismetSystemLibrary.PrintString` "invalid in bp" true true (struct :`G` 0.66 :`B` 1.0 :`A` 1.0) 5.0))))

(fn `AddEquip`
  (params (`finishAppearancePrep?` :type Boolean) (styleIndex :type Byte) (colorIndex :type Byte))
  (locals (localPickupItemInfo :type "/Game/GameSystem/Structures/S_PickupItemInfo Structure") (localEquipPaperSprite :type "PaperSpriteComponent Object Reference") (localTranslucentPriority :type Integer :default 14) (l_styleIndex :type Byte) (l_colorIndex :type Byte))
  (bind _localequippapersprite (`local.localEquipPaperSprite`))
  (bind _localequippapersprite_2 (`local.localEquipPaperSprite`))
  (bind _creationstr (`self.creationStr`))
  (bind (_lefts _rights) (`KismetStringLibrary.Split` (`self.appearanceString`) ":"))
  (bind _returnvalue (`KismetStringLibrary.IsEmpty` _creationstr))
  (bind _returnvalue_2 (`KismetStringLibrary.Conv_StringToName` _rights))
  (bind _returnvalue_3 (`KismetStringLibrary.Conv_StringToName` _lefts))
  (set `local.l_styleIndex` styleIndex)
  (set `local.l_colorIndex` colorIndex)
  (if `finishAppearancePrep?`
    (if _returnvalue
      (bind _facestyle (`self.getCorrectTextureStyle` (`self.AllFaceStylesDT`) (`local.l_styleIndex`) (`local.l_colorIndex`) "face" :!label _label)
        (:`then`
          (bind _returnvalue_4 (`|GetDataTableRow` "/Game/GameSystem/DataTables/Equipments/EquipmentTranslucentPriorities_DT.EquipmentTranslucentPriorities_DT" "Idle/Alert")
            (:`then`
              (set `local.localTranslucentPriority` (`.FaceExpression_15_F59FFFA54270D8D37998EFAF115E3755` (break `/Game/GameSystem/Structures/S_TranslucentPriorityPerAnimation` _returnvalue_4)))
              (bind _returnvalue_5 (`AddComponent|NODE_AddPaperSpriteComponent-1`))
              (bind _output_get (set `local.localEquipPaperSprite` _returnvalue_5))
              (bind _returnvalue_6 (`PaperSpriteComponent.SetSprite` _output_get (`.FaceStyleSprite_5_B05C003045BA726A7F7672AC8ACA7F95` (break `/Game/GameSystem/Structures/S_FaceStyle` _facestyle))))
              (if _returnvalue_6
                (`PrimitiveComponent.SetTranslucentSortPriority` _localequippapersprite (`local.localTranslucentPriority`))
                (`SceneComponent.K2_AttachToComponent` _localequippapersprite (`self.PaperFlipbook`) "FaceExpression" "KeepRelative" "SnapToTarget" "KeepRelative" true)))))
        (:`RowNotFound`
          _))
      (if (not (or (`self.hasHat?`) (not _returnvalue)))
        (bind (_facestyle_2 _hairstyle) (`self.getCorrectTextureStyle` (`self.AllHairStylesDT`) (`local.l_styleIndex`) (`local.l_colorIndex`) "hair" :!label _label_2)
          (:`then`
            (bind _returnvalue_7 (`|GetDataTableRow` "/Game/GameSystem/DataTables/Equipments/EquipmentTranslucentPriorities_DT.EquipmentTranslucentPriorities_DT" "Idle/Alert")
              (:`then`
                (set `local.localTranslucentPriority` (`.Hat_2_1C0BF060498702910BE68CA1D73C6BB1` (break `/Game/GameSystem/Structures/S_TranslucentPriorityPerAnimation` _returnvalue_7)))
                (bind _returnvalue_8 (`AddComponent|NODE_AddPaperSpriteComponent-2`))
                (bind _output_get_2 (set `local.localEquipPaperSprite` _returnvalue_8))
                (bind _returnvalue_9 (`PaperSpriteComponent.SetSprite` _output_get_2 (`.Normal_4_817D3FC64F48380CF577088627AE6687` (break `/Game/GameSystem/Structures/S_HairStyleSprites` _hairstyle))))
                (if _returnvalue_9
                  (`PrimitiveComponent.SetTranslucentSortPriority` _localequippapersprite_2 (`local.localTranslucentPriority`))
                  (`SceneComponent.K2_AttachToComponent` _localequippapersprite_2 (`self.PaperFlipbook`) "Hat" "KeepRelative" "SnapToTarget" "KeepRelative" true)))))))
      (else
        (switch `string` _creationstr
          (:`Face`
            (goto _label))
          (:`Hair`
            (goto _label_2)))))
    (else
      (switch `string` _lefts ; apparently , there is no option to select a data table dynamically with just a name...
        (:`Hat`
          (bind _returnvalue_10 (`|GetDataTableRow` "/Game/GameSystem/DataTables/Equipments/HatsDataTable.HatsDataTable" _returnvalue_2)
            (:`then`
              (set `local.localPickupItemInfo` _returnvalue_10)
              (bind _returnvalue_11 (`|GetDataTableRow` "/Game/GameSystem/DataTables/Equipments/EquipmentTranslucentPriorities_DT.EquipmentTranslucentPriorities_DT" "Idle/Alert")
                (:`then`
                  (set `local.localTranslucentPriority` (`.Hat_2_1C0BF060498702910BE68CA1D73C6BB1` (break `/Game/GameSystem/Structures/S_TranslucentPriorityPerAnimation` _returnvalue_11))))
                (:`RowNotFound`
                  _))
              (set `self.hasHat?` true))))
        (:`Secondary`
          (bind _returnvalue_12 (`|GetDataTableRow` "/Game/GameSystem/DataTables/Equipments/SecondaryDataTable.SecondaryDataTable" _returnvalue_2)
            (:`then`
              (set `local.localPickupItemInfo` _returnvalue_12)
              (bind _returnvalue_13 (`|GetDataTableRow` "/Game/GameSystem/DataTables/Equipments/EquipmentTranslucentPriorities_DT.EquipmentTranslucentPriorities_DT" "Idle/Alert")
                (:`then`
                  (set `local.localTranslucentPriority` (`.Secondary_35_F0D4668041B5B4E060CB59BFC63FB44D` (break `/Game/GameSystem/Structures/S_TranslucentPriorityPerAnimation` _returnvalue_13))))
                (:`RowNotFound`
                  _)))))
        (:`Weapon`
          (bind _returnvalue_14 (`|GetDataTableRow` "/Game/GameSystem/DataTables/Equipments/WeaponsDataTable.WeaponsDataTable" _returnvalue_2)
            (:`then`
              (set `local.localPickupItemInfo` _returnvalue_14)
              (bind _returnvalue_15 (`|GetDataTableRow` "/Game/GameSystem/DataTables/Equipments/EquipmentTranslucentPriorities_DT.EquipmentTranslucentPriorities_DT" "Idle/Alert")
                (:`then`
                  (set `local.localTranslucentPriority` (`.Weapon_43_18A3B83C43D8BCDEB4CFAEA353F9EB5B` (break `/Game/GameSystem/Structures/S_TranslucentPriorityPerAnimation` _returnvalue_15))))
                (:`RowNotFound`
                  _)))))
        (:`Ring`
          (bind _returnvalue_16 (`|GetDataTableRow` "/Game/GameSystem/DataTables/Equipments/RingsDataTable.RingsDataTable" _returnvalue_2)
            (:`then`
              (set `local.localPickupItemInfo` _returnvalue_16)
              (bind _returnvalue_17 (`|GetDataTableRow` "/Game/GameSystem/DataTables/Equipments/EquipmentTranslucentPriorities_DT.EquipmentTranslucentPriorities_DT" "Idle/Alert")
                (:`then`
                  (set `local.localTranslucentPriority` (`.Ring14_30_178ED24D453F1A1AA3C2A68F056ADE75` (break `/Game/GameSystem/Structures/S_TranslucentPriorityPerAnimation` _returnvalue_17))))
                (:`RowNotFound`
                  _))))))
      (bind _returnvalue_18 (`AddComponent|NODE_AddPaperSpriteComponent-0`))
      (bind _output_get_3 (set `local.localEquipPaperSprite` _returnvalue_18))
      (bind _returnvalue_19 (`PaperSpriteComponent.SetSprite` _output_get_3 (`.idle_13_DC0BC7C8487E640A26DF609C1DC7BE0D` (break `/Game/GameSystem/Structures/S_EquipmentAnimations` (`.EquipSpriteAnimations_103_BCBD55964CF0C4339EBE32BC114E8573` (break `/Game/GameSystem/Structures/S_EquipInfo` (`.EquipInfoStruct_8_5EAC3381467C0B4FDFDE06AC9CDEBDC2` (break `/Game/GameSystem/Structures/S_PickupItemInfo` (`local.localPickupItemInfo`)))))))))
      (if _returnvalue_19
        (if (`SceneComponent.DoesSocketExist` (`self.PaperFlipbook`) _returnvalue_3)
          (`PrimitiveComponent.SetTranslucentSortPriority` (`local.localEquipPaperSprite`) (`local.localTranslucentPriority`))
          (`SceneComponent.K2_AttachToComponent` (`local.localEquipPaperSprite`) (`self.PaperFlipbook`) _returnvalue_3 "KeepRelative" "KeepRelative" "KeepRelative" true))))))

(fn `UserConstructionScript`)