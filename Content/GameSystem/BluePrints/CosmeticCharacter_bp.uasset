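; Cosmetic 2D character for the creation and selection screens, dressing a PaperFlipbook with socket-attached sprites.
; AddEquip parses "Type:Value" appearance strings, creating equipment sprite components or storing face and hair style-color indices.
; Its finishing pass resolves face and hair through nested gender, style and color data tables, reusing existing socket sprites.
; Hair shares the Hat socket, so a hat suppresses it; sort priorities come from a data table.
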(event `self.ReceiveBeginPlay`
  (`PrimitiveComponent.SetTranslucentSortPriority` (`self.PaperFlipbook`) 13))

(fn `AddEquip`
  (params (`finishAppearancePrep?` :type Boolean) (styleIndex :type Byte) (colorIndex :type Byte))
  (locals (localPickupItemInfo :type "/Game/GameSystem/Structures/S_PickupItemInfo Structure") (localEquipPaperSprite :type "PaperSpriteComponent Object Reference") (localTranslucentPriority :type Integer :default 14) (l_styleIndex :type Byte) (l_colorIndex :type Byte))
  (bind _localtranslucentpriority (`local.localTranslucentPriority`))
  (bind _localequippapersprite (`local.localEquipPaperSprite`))
  (bind _localequippapersprite_2 (`local.localEquipPaperSprite`))
  (bind _l_styleindex (`local.l_styleIndex`))
  (bind _l_colorindex (`local.l_colorIndex`))
  (bind _localtranslucentpriority_2 (`local.localTranslucentPriority`))
  (bind _creationstr (`self.creationStr`))
  (bind (_lefts _rights) (`KismetStringLibrary.Split` (`self.appearanceString`) ":"))
  (bind _returnvalue (`KismetStringLibrary.IsEmpty` _creationstr))
  (bind _returnvalue_2 (`KismetStringLibrary.Conv_StringToName` _rights))
  (bind _returnvalue_3 (`KismetStringLibrary.Conv_StringToName` _lefts))
  (bind (_lefts_2 _rights_2 _returnvalue_4) (`KismetStringLibrary.Split` _rights "-"))
  (bind _returnvalue_5 (`KismetMathLibrary.Conv_IntToByte` (- (`KismetStringLibrary.GetCharacterAsNumber` _lefts_2) 48)))
  (bind _returnvalue_6 (`KismetMathLibrary.Conv_IntToByte` (- (`KismetStringLibrary.GetCharacterAsNumber` _rights_2) 48)))
  (set `local.l_styleIndex` styleIndex)
  (set `local.l_colorIndex` colorIndex)
  (if `finishAppearancePrep?`
    (if _returnvalue
      ;[1 1 1] FaceStyle
      (bind _facestyle (`self.getCorrectTextureStyle` (`self.AllFaceStylesDT`) (`self.faceStyleIndex`) (`self.faceStyleColorIndex`) "face" :!label _label)
        (:`then`
          (bind (_hattpriority _facetpriority _aspaper_sprite_component) (`self.setCosmeticObjVars` "FaceExpression" :!label _label_2)
            (:`then`
              (set `local.localTranslucentPriority` _facetpriority)
              (goto _label_2 :!via `execute2`))
            (:`compExists`
              (bind (_facestylename _facestylesprite) (break `/Game/GameSystem/Structures/S_FaceStyle` _facestyle))
              (bind _returnvalue_7 (`PaperSpriteComponent.SetSprite` _aspaper_sprite_component _facestylesprite))
              (if _returnvalue_7
                (`PrimitiveComponent.SetTranslucentSortPriority` _aspaper_sprite_component _localtranslucentpriority_2)
                ;[1 1 1] HairStyle
                (if (not (or (`self.hasHat?`) (not _returnvalue))) :!label _label_3
                  (bind (_facestyle_2 _hairstyle) (`self.getCorrectTextureStyle` (`self.AllHairStylesDT`) (`self.hairStyleIndex`) (`self.hairStyleColorIndex`) "hair" :!label _label_4)
                    (:`then`
                      (bind (_hattpriority_2 _facetpriority_2 _aspaper_sprite_component_2) (`self.setCosmeticObjVars` "Hat" :!label _label_5)
                        (:`then`
                          (set `local.localTranslucentPriority` _hattpriority_2)
                          (goto _label_5 :!via `execute2`))
                        (:`compExists`
                          (bind (_hairstylename _normal) (break `/Game/GameSystem/Structures/S_HairStyleSprites` _hairstyle))
                          (bind _returnvalue_8 (`PaperSpriteComponent.SetSprite` _aspaper_sprite_component_2 _normal))
                          (if _returnvalue_8
                            (`PrimitiveComponent.SetTranslucentSortPriority` _aspaper_sprite_component_2 _localtranslucentpriority)))
                        (:`notExists`
                          (bind _returnvalue_9 (`AddComponent|NODE_AddPaperSpriteComponent-2`))
                          (bind _output_get (set `local.localEquipPaperSprite` _returnvalue_9))
                          (bind _returnvalue_10 (`PaperSpriteComponent.SetSprite` _output_get _normal))
                          (if _returnvalue_10
                            (`PrimitiveComponent.SetTranslucentSortPriority` _localequippapersprite_2 _localtranslucentpriority)
                            (`SceneComponent.K2_AttachToComponent` _localequippapersprite_2 (`self.PaperFlipbook`) "Hat" "KeepRelative" "SnapToTarget" "KeepRelative" true)))))))))
            (:`notExists`
              (bind _returnvalue_11 (`AddComponent|NODE_AddPaperSpriteComponent-1`))
              (bind _output_get_2 (set `local.localEquipPaperSprite` _returnvalue_11))
              (bind _returnvalue_12 (`PaperSpriteComponent.SetSprite` _output_get_2 _facestylesprite))
              (if _returnvalue_12
                (`PrimitiveComponent.SetTranslucentSortPriority` _localequippapersprite _localtranslucentpriority_2)
                (`SceneComponent.K2_AttachToComponent` _localequippapersprite (`self.PaperFlipbook`) "FaceExpression" "KeepRelative" "SnapToTarget" "KeepRelative" true)
                (goto _label_3)
                (else
                  (goto _label_3))))))
        (:`RowNotFound`
          (bind _returnvalue_13 (`|GetDataTableRow` "/Game/GameSystem/DataTables/Character/Styles/Female/Faces/FemaleFaceStyle1_DT.FemaleFaceStyle1_DT" "DefaultFemaleFaceStyle") ; default
            (:`then`
              (bind (_hattpriority_3 _facetpriority_3 _aspaper_sprite_component_3) (`self.setCosmeticObjVars` "FaceExpression" :!label _label_6)
                (:`then`
                  (set `local.localTranslucentPriority` _facetpriority_3)
                  (goto _label_6 :!via `execute2`))
                (:`compExists`
                  (bind (_facestylename_2 _facestylesprite_2) (break `/Game/GameSystem/Structures/S_FaceStyle` _returnvalue_13))
                  (bind _returnvalue_14 (`PaperSpriteComponent.SetSprite` _aspaper_sprite_component_3 _facestylesprite_2))
                  (if _returnvalue_14
                    (`PrimitiveComponent.SetTranslucentSortPriority` _aspaper_sprite_component_3 (`local.localTranslucentPriority`))
                    (goto _label_3)))
                (:`notExists`
                  (bind _returnvalue_15 (`AddComponent|NODE_AddPaperSpriteComponent-4`))
                  (bind _output_get_3 (set `local.localEquipPaperSprite` _returnvalue_15))
                  (bind _returnvalue_16 (`PaperSpriteComponent.SetSprite` _output_get_3 _facestylesprite_2))
                  (if _returnvalue_16
                    (`PrimitiveComponent.SetTranslucentSortPriority` _localequippapersprite _localtranslucentpriority_2)
                    (`SceneComponent.K2_AttachToComponent` _localequippapersprite (`self.PaperFlipbook`) "FaceExpression" "KeepRelative" "SnapToTarget" "KeepRelative" true)
                    (goto _label_3)
                    (else
                      (goto _label_3))))))
            (:`RowNotFound`
              (goto _label_3)))))
      (else
        ;[1 1 1] should get to this part only from a creation screen character, not from the selection screen characters
        (switch `string` _creationstr
          (:`Face`
            (set `self.faceStyleIndex` _l_styleindex)
            (set `self.faceStyleColorIndex` _l_colorindex)
            (goto _label))
          (:`Hair`
            (set `self.hairStyleIndex` _l_styleindex)
            (set `self.hairStyleColorIndex` _l_colorindex)
            (goto _label_4)))))
    (else
      (switch `string` _lefts ; apparently , there is no option to select a data table dynamically with just a name...
        (:`Hat`
          (bind _returnvalue_17 (`|GetDataTableRow` "/Game/GameSystem/DataTables/Equipments/HatsDataTable.HatsDataTable" _returnvalue_2)
            (:`then`
              (set `local.localPickupItemInfo` _returnvalue_17)
              (bind _returnvalue_18 (`|GetDataTableRow` "/Game/GameSystem/DataTables/Equipments/EquipmentTranslucentPriorities_DT.EquipmentTranslucentPriorities_DT" "Idle/Alert")
                (:`then`
                  (set `local.localTranslucentPriority` (`.Hat_2_1C0BF060498702910BE68CA1D73C6BB1` (break `/Game/GameSystem/Structures/S_TranslucentPriorityPerAnimation` _returnvalue_18))))
                (:`RowNotFound`
                  _))
              (set `self.hasHat?` true)
              (bind _returnvalue_19 (`AddComponent|NODE_AddPaperSpriteComponent-0` :!label _label_7))
              (bind _output_get_4 (set `local.localEquipPaperSprite` _returnvalue_19))
              (bind _returnvalue_20 (`PaperSpriteComponent.SetSprite` _output_get_4 null))
              (if _returnvalue_20
                (if (`SceneComponent.DoesSocketExist` (`self.PaperFlipbook`) _returnvalue_3)
                  (`PrimitiveComponent.SetTranslucentSortPriority` (`local.localEquipPaperSprite`) (`local.localTranslucentPriority`))
                  (`SceneComponent.K2_AttachToComponent` (`local.localEquipPaperSprite`) (`self.PaperFlipbook`) _returnvalue_3 "KeepRelative" "KeepRelative" "KeepRelative" true))))))
        (:`Secondary`
          (bind _returnvalue_21 (`|GetDataTableRow` "/Game/GameSystem/DataTables/Equipments/SecondaryDataTable.SecondaryDataTable" _returnvalue_2)
            (:`then`
              (set `local.localPickupItemInfo` _returnvalue_21)
              (bind _returnvalue_22 (`|GetDataTableRow` "/Game/GameSystem/DataTables/Equipments/EquipmentTranslucentPriorities_DT.EquipmentTranslucentPriorities_DT" "Idle/Alert")
                (:`then`
                  (set `local.localTranslucentPriority` (`.Secondary_35_F0D4668041B5B4E060CB59BFC63FB44D` (break `/Game/GameSystem/Structures/S_TranslucentPriorityPerAnimation` _returnvalue_22)))
                  (goto _label_7))
                (:`RowNotFound`
                  (goto _label_7))))))
        (:`Weapon`
          (bind _returnvalue_23 (`|GetDataTableRow` "/Game/GameSystem/DataTables/Equipments/WeaponsDataTable.WeaponsDataTable" _returnvalue_2)
            (:`then`
              (set `local.localPickupItemInfo` _returnvalue_23)
              (bind _returnvalue_24 (`|GetDataTableRow` "/Game/GameSystem/DataTables/Equipments/EquipmentTranslucentPriorities_DT.EquipmentTranslucentPriorities_DT" "Idle/Alert")
                (:`then`
                  (set `local.localTranslucentPriority` (`.Weapon_43_18A3B83C43D8BCDEB4CFAEA353F9EB5B` (break `/Game/GameSystem/Structures/S_TranslucentPriorityPerAnimation` _returnvalue_24)))
                  (goto _label_7))
                (:`RowNotFound`
                  (goto _label_7))))))
        (:`Ring`
          (bind _returnvalue_25 (`|GetDataTableRow` "/Game/GameSystem/DataTables/Equipments/RingsDataTable.RingsDataTable" _returnvalue_2)
            (:`then`
              (set `local.localPickupItemInfo` _returnvalue_25)
              (bind _returnvalue_26 (`|GetDataTableRow` "/Game/GameSystem/DataTables/Equipments/EquipmentTranslucentPriorities_DT.EquipmentTranslucentPriorities_DT" "Idle/Alert")
                (:`then`
                  (set `local.localTranslucentPriority` (`.Ring14_30_178ED24D453F1A1AA3C2A68F056ADE75` (break `/Game/GameSystem/Structures/S_TranslucentPriorityPerAnimation` _returnvalue_26)))
                  (goto _label_7))
                (:`RowNotFound`
                  (goto _label_7))))))
        (:`Face`
          (if _returnvalue_4
            (set `self.faceStyleIndex` _returnvalue_5)
            (set `self.faceStyleColorIndex` _returnvalue_6)))
        (:`Hair`
          (if _returnvalue_4
            (set `self.hairStyleIndex` _returnvalue_5)
            (set `self.hairStyleColorIndex` _returnvalue_6)))))))

(fn `FuncGetSpriteCompBySocketName`
  (params (SocketName :type Name))
  (returns (`AsPaper Sprite Component` :type "PaperSpriteComponent Object Reference") (`Success?` :type Boolean))
  (for _array_element (`SceneComponent.GetChildrenComponents` (`self.PaperFlipbook`) false)
    (bind _aspaper_sprite_component (cast `PaperSpriteComponent` _array_element))
    (if (== SocketName (`SceneComponent.GetAttachSocketName` _aspaper_sprite_component))
      (return _aspaper_sprite_component true)))
  (return null false))

(fn `UserConstructionScript`)