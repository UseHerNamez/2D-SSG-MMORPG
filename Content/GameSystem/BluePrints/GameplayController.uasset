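; Player controller for a 2D quest game that tracks the player's quest progress and drives NPC quest indicators.
; Server-named events advance quest status and grant EXP, currency or item rewards through the character interface, while monster objective counters move quests to waiting-for-completion.
; Indicators combine quest states by priority with DataTable level requirements, reaching NPCs by interface.
; It also handles animated hand cursors, currency updates and a loading widget.
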(event `ChangeCharQuestWidgetBool`
  (params (value :type Boolean))
  (bind _returnvalue (`self.K2_GetPawn`))
  (`self.check interface use` _returnvalue)
  (message `/Game/GameSystem/BluePrints/BPInterface_Char.Change Quest Dialog bool value interface` _returnvalue value))

(event `Event_CheckQuestIndicatorStatus_Serv`
  (params (`NPC name` :type Name) (NPC_REF :type "Actor Object Reference"))
  (bind _final_status (`self.CheckQuestIndicator` `NPC name`))
  (if (`KismetSystemLibrary.DoesImplementInterface` NPC_REF "/Game/GameSystem/BluePrints/BPInterface_NPC.BPInterface_NPC_C")
    (message `/Game/GameSystem/BluePrints/BPInterface_NPC.call change quest indicator func interface` NPC_REF _final_status)))

(event `self.ReceiveBeginPlay`
  (set `self.bShowMouseCursor` true))

(event `OnUpdateCurrency`
  (params (Rakins :type "/Game/GameSystem/Structures/Rakins_Struct Structure") (`Premium Rakins` :type Boolean))
  (bind _returnvalue (`self.K2_GetPawn`))
  (if (`KismetSystemLibrary.DoesImplementInterface` _returnvalue)
    (message `/Game/GameSystem/BluePrints/BPInterface_Char.set rakins interface` _returnvalue Rakins)))

(event `Key|LeftMouseButton` :consume false
  (params (Key :type "Key Structure"))
  (:`Pressed`
    (set `self.leftClickDown?` true)
    (set `self.CurrentMouseCursor` "Hand" :!label _label)
    (`KismetSystemLibrary.Delay` 0.2)
    (if (`self.leftClickDown?`)
      (set `self.CurrentMouseCursor` "GrabHand")
      (`KismetSystemLibrary.Delay` 0.2)
      (if (`self.leftClickDown?`)
        (set `self.CurrentMouseCursor` "GrabHandClosed")
        (`KismetSystemLibrary.Delay` 0.2)
        (if (`self.leftClickDown?`)
          (goto _label)))))
  (:`Released`
    (set `self.leftClickDown?` false)
    (set `self.CurrentMouseCursor` "Default")))

(event `ChangeQuestStatus_Serv`
  (params (QuestToChange :type "/Game/GameSystem/Structures/S_PlayerQuestsStatus Structure") (questNumber :type Integer) (NPC_REF :type "Actor Object Reference"))
  (bind _returnvalue (`self.K2_GetPawn`))
  (bind _allopenedquestsstatusesandinfo (`self.AllOpenedQuestsStatusesAndInfo`))
  (bind (_npcname _npcsprite _allquestsinfo) (break `/Game/GameSystem/Structures/S_QuestNPC_Info` (`.QuestNPCInfo_17_3885FF354345E935625AB2BBB2F0F311` (break `/Game/GameSystem/Structures/S_PlayerQuestsStatus` QuestToChange))))
  (for (_array_element _array_index) _allopenedquestsstatusesandinfo
    (bind (_questnpcinfo _currentquestsstatus) (break `/Game/GameSystem/Structures/S_PlayerQuestsStatus` _array_element))
    (if (== (`.NPCName_2_408B2968443A3DDDF01962807A38688E` (break `/Game/GameSystem/Structures/S_QuestNPC_Info` _questnpcinfo)) _npcname)
      (bind _output (`|GetArrayItem` _currentquestsstatus questNumber))
      (bind (_queststatus _questnumber) (break `/Game/GameSystem/Structures/S_currentSingleQuestStatus` _output))
      (if (`|EnumEquality` _queststatus "NewEnumerator0")
        (bind _output_2 (`|GetArrayItem` (`.currentQuestsStatus_18_53F412FC4D3098498036FC8409A7E086` (break `/Game/GameSystem/Structures/S_PlayerQuestsStatus` (`|GetArrayItem` _allopenedquestsstatusesandinfo _array_index))) questNumber))
        (setmembers `/Game/GameSystem/Structures/S_currentSingleQuestStatus` :`StructRef` _output_2 :`questStatus` (cast `/Game/GameSystem/Enums/E_PlayerQuestsStatus` (+ (`.questStatus_6_397184FB4D562F74F7E2C780174B7B97` (break `/Game/GameSystem/Structures/S_currentSingleQuestStatus` _output_2)) 1)) :`questNumber` _questnumber)
        (`self.Event_CheckQuestIndicatorStatus_Serv` _npcname NPC_REF)
        (break)
        (else
          (if (== (- (`KismetArrayLibrary.Array_Length` _currentquestsstatus) 1) _questnumber)
            (bind _returnvalue_2 (cast `/Game/GameSystem/Enums/E_PlayerQuestsStatus` (+ _queststatus 1)))
            (setmembers `/Game/GameSystem/Structures/S_currentSingleQuestStatus` :`StructRef` _output :`questStatus` _returnvalue_2 :`questNumber` _questnumber)
            (else
              (setmembers `/Game/GameSystem/Structures/S_currentSingleQuestStatus` :`StructRef` _output :`questStatus` _returnvalue_2 :`questNumber` (+ _questnumber 1))))
          (`self.Event_CheckQuestIndicatorStatus_Serv` _npcname NPC_REF)
          (if (`KismetSystemLibrary.DoesImplementInterface` _returnvalue "/Game/GameSystem/BluePrints/BPInterface_Char.BPInterface_Char_C")
            (for _array_element_2 (`.ArrayOfRewards_33_2AD633A5429B6E986EFDD4830716A184` (break `/Game/GameSystem/Structures/S_QuestInfo` (`|GetArrayItem` _allquestsinfo questNumber)))
              (bind (_rewardtype _iteminfo _rakinamount _exp) (break `/Game/GameSystem/Structures/S_QuestRewards` _array_element_2))
              (switch `/Game/GameSystem/Enums/E_QuestRewardTypes` _rewardtype
                (:`NewEnumerator0`
                  (message `/Game/GameSystem/BluePrints/BPInterface_Char.Gain EXP interface` _returnvalue _exp))
                (:`NewEnumerator1`
                  (message `/Game/GameSystem/BluePrints/BPInterface_Char.add Item to inventory interface` _returnvalue true _rakinamount (struct)))
                (:`NewEnumerator2`
                  (message `/Game/GameSystem/BluePrints/BPInterface_Char.add Item to inventory interface` _returnvalue true (struct) _iteminfo))))))))))

(event `/Game/BPInterface_GameplayController.call change quest status func interface`
  (params (`quest status` :type "/Game/GameSystem/Structures/S_PlayerQuestsStatus Structure") (`quest num` :type Integer) (`npc REF` :type "Actor Object Reference"))
  (`self.ChangeQuestStatus_Serv` `quest status` `quest num` `npc REF`))

(event `/Game/BPInterface_GameplayController.call check quest indicator func interface`
  (params (`npc ref` :type "Actor Object Reference") (name :type Name))
  (`self.Event_CheckQuestIndicatorStatus_Serv` name `npc ref`))

(event `/Game/BPInterface_GameplayController.set translucent ID`
  (params (`Id in` :type Integer))
  (set `self.TranslucentID` `Id in`))

(event `self.ShowLoadingWidget`
  (bind _loadingwidget (`self.LoadingWidget`))
  ;[1 1 1] LoadingWidget
  (if (not (`KismetSystemLibrary.IsValid` _loadingwidget))
    (bind _returnvalue (`|CreateWidget` "/Game/GameSystem/Widgets/LoadingWidget.LoadingWidget_C"))
    (bind _output_get (set `self.LoadingWidget` _returnvalue))
    (`UserWidget.AddToViewport` _output_get 0))
  (`Widget.SetVisibility` _loadingwidget "HitTestInvisible"))

(event `self.HideLoadingWidget`
  ;[1 1 1] LoadingWidget
  (`Widget.SetVisibility` (`self.LoadingWidget`) "Hidden"))

(event `self.ShowErrorWidget`
  (params (ErrorMessage :type String))
  ;[1 1 1] Error Widget
)

(fn `Check if Monster in Ongoing Quest`
  (params (questInfo :type "Array of /Game/GameSystem/Structures/S_monsterQuestsParticipate Structure"))
  (bind _allopenedquestsstatusesandinfo (`self.AllOpenedQuestsStatusesAndInfo`))
  (for _array_element questInfo
    (for (_array_element_2 _array_index) _allopenedquestsstatusesandinfo :!label _label
      (bind (_questnpcinfo _currentquestsstatus) (break `/Game/GameSystem/Structures/S_PlayerQuestsStatus` _array_element_2))
      (bind (_npcname _npcsprite _allquestsinfo) (break `/Game/GameSystem/Structures/S_QuestNPC_Info` _questnpcinfo))
      (bind (_npcname_2 _questnum) (break `/Game/GameSystem/Structures/S_monsterQuestsParticipate` _array_element))
      (if (== _npcname _npcname_2)
        (switch `/Game/GameSystem/Enums/E_PlayerQuestsStatus` (`.questStatus_6_397184FB4D562F74F7E2C780174B7B97` (break `/Game/GameSystem/Structures/S_currentSingleQuestStatus` (`|GetArrayItem` _currentquestsstatus _questnum)))
          (:`NewEnumerator0`
            (break))
          (:`NewEnumerator1`
            (bind _output (`|GetArrayItem` (`.currentQuestsStatus_18_53F412FC4D3098498036FC8409A7E086` (break `/Game/GameSystem/Structures/S_PlayerQuestsStatus` (`|GetArrayItem` _allopenedquestsstatusesandinfo _array_index))) _questnum))
            (bind ((`counterOfObjective_10_53FF6B384B609BD51CE4C699CA73B22A` _counterofobjective)) (break `/Game/GameSystem/Structures/S_currentSingleQuestStatus` _output))
            (setmembers `/Game/GameSystem/Structures/S_currentSingleQuestStatus` :`StructRef` _output :`counterOfObjective` (+ _counterofobjective 1))
            (if (== (`.Amount_5_2EBB3EC348968916FE557AB0B964480D` (break `/Game/GameSystem/Structures/S_QuestMissionTypeAndInfo` (`|GetArrayItem` (`.arrayOfMissionsTypeAndInfo_22_FFD67E9042B4BE27A44EFBB5C885C595` (break `/Game/GameSystem/Structures/S_QuestInfo` (`|GetArrayItem` _allquestsinfo _questnum)))))) _counterofobjective)
              (setmembers `/Game/GameSystem/Structures/S_currentSingleQuestStatus` :`StructRef` _output :`questStatus` "NewEnumerator2")
              (bind _as2dgame_state_base (cast `/Game/2DSideScrollerBP/Blueprints/2DGameStateBase` (`GameplayStatics.GetGameState`)))
              (for _array_element_3 (`/Game/2DSideScrollerBP/Blueprints/2DGameStateBase.arrayOfNpcREFs` _as2dgame_state_base)
                (bind (_npcref _npcname_3) (break `/Game/GameSystem/Structures/S_NpcREFbyName` _array_element_3))
                (if (== _npcname_3 _npcname_2)
                  (`self.Event_CheckQuestIndicatorStatus_Serv` _npcname_3 _npcref)
                  (goto _label :!via `Break`)))
              (else
                (break))))
          (:`NewEnumerator2`
            (break))
          (:`NewEnumerator3`
            (break))))))
  (return))

(fn `CheckQuestIndicator`
  (params (`NPC name` :type Name))
  (returns (`final status` :type "/Game/GameSystem/Enums/E_PlayerQuestsStatus Enum"))
  (locals (finalQuestStatusToShow :type "/Game/GameSystem/Enums/E_PlayerQuestsStatus Enum") (NPCNamesInExistingQuestsArr :type "Array of Name") (lowetREQLevelCurrQuest :type Integer))
  (bind _returnvalue (`self.K2_GetPawn`))
  (bind _finalqueststatustoshow (`local.finalQuestStatusToShow`))
  (bind _returnvalue_2 (`|EnumEquality` _finalqueststatustoshow "NewEnumerator2"))
  (set `local.finalQuestStatusToShow` "NewEnumerator3")
  (for _array_element (`self.AllOpenedQuestsStatusesAndInfo`)
    (bind (_questnpcinfo _currentquestsstatus) (break `/Game/GameSystem/Structures/S_PlayerQuestsStatus` _array_element))
    (if (== (`.NPCName_2_408B2968443A3DDDF01962807A38688E` (break `/Game/GameSystem/Structures/S_QuestNPC_Info` _questnpcinfo)) `NPC name`)
      (`KismetArrayLibrary.Array_AddUnique` (`local.NPCNamesInExistingQuestsArr`) `NPC name`)
      (for _array_element_2 _currentquestsstatus
        (switch `/Game/GameSystem/Enums/E_PlayerQuestsStatus` (`.questStatus_6_397184FB4D562F74F7E2C780174B7B97` (break `/Game/GameSystem/Structures/S_currentSingleQuestStatus` _array_element_2))
          (:`NewEnumerator0`
            (if (not _returnvalue_2)
              (set `local.finalQuestStatusToShow` "NewEnumerator0")))
          (:`NewEnumerator1`
            (if (not (or (`|EnumEquality` _finalqueststatustoshow "NewEnumerator0") _returnvalue_2))
              (set `local.finalQuestStatusToShow` "NewEnumerator1")))
          (:`NewEnumerator2`
            (set `local.finalQuestStatusToShow` "NewEnumerator2"))))
      (break)))
  (bind _as2dgame_state_base (cast `/Game/2DSideScrollerBP/Blueprints/2DGameStateBase` (`GameplayStatics.GetGameState`)))
  (for _array_element_3 (`/Game/2DSideScrollerBP/Blueprints/2DGameStateBase.arrayOfNpcREFs` _as2dgame_state_base)
    (bind (_npcref _npcname) (break `/Game/GameSystem/Structures/S_NpcREFbyName` _array_element_3))
    (if (== (`KismetArrayLibrary.Array_Find` (`local.NPCNamesInExistingQuestsArr`) _npcname) -1)
      (`self.check interface use` _returnvalue)
      (bind _level (message `/Game/GameSystem/BluePrints/BPInterface_Char.get char LVL interface` _returnvalue))
      (bind _returnvalue_3 (`|GetDataTableRow` "/Game/GameSystem/DataTables/AllQuestsInfos_DT.AllQuestsInfos_DT" _npcname)
        (:`then`
          (bind (_npcname_2 _npcsprite _allquestsinfo) (break `/Game/GameSystem/Structures/S_QuestNPC_Info` _returnvalue_3))
          (set `local.lowetREQLevelCurrQuest` (`.levelREQ_26_E2B13FF4410A3E1F141C1FB161E1FC3E` (break `/Game/GameSystem/Structures/S_QuestInfo` (`|GetArrayItem` _allquestsinfo))))
          (for _array_element_4 _allquestsinfo
            (bind ((`levelREQ_26_E2B13FF4410A3E1F141C1FB161E1FC3E` _levelreq)) (break `/Game/GameSystem/Structures/S_QuestInfo` _array_element_4))
            (if (< _levelreq (`local.lowetREQLevelCurrQuest`))
              (set `local.lowetREQLevelCurrQuest` _levelreq)))
          (if (not (> (`local.lowetREQLevelCurrQuest`) _level))
            (set `local.finalQuestStatusToShow` "NewEnumerator0"))))))
  (return (`local.finalQuestStatusToShow`)))

(fn `get paper char ref interface`
  (returns (`char ref` :type "PaperCharacter Object Reference"))
  (bind _aspaper_character (cast `PaperCharacter` (`self.K2_GetPawn`)))
  (return _aspaper_character))

(fn `get translucent ID`
  (returns (`T id` :type Integer))
  (return (`self.TranslucentID`)))

(fn `UserConstructionScript`)