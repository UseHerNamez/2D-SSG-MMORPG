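; Blueprint Interface for the player character, letting other objects call it without casting.
; Covers combat damage, EXP, level, stats and AP, inventory, equipment and item use, climbing and animation multicasts, chat bubbles, and widget access.
; A large group handles expedition (party) invitations, membership, leadership, kicks, map changes and logout, with server and client variants.
; Functions are declarations only, with empty or default returns, so implementers supply all logic.
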(fn `Add AP Stats interface`
  (params (`Which stat?` :type "/Game/GameSystem/Enums/E_APStats Enum" :default "NewEnumerator0")))

(fn `add Item to inventory interface`
  (params (`notification?` :type Boolean) (`rakins info` :type "/Game/GameSystem/Structures/Rakins_Struct Structure") (`item info` :type "/Game/GameSystem/Structures/S_PickupItemInfo Structure")))

(fn `AddNewXpedMemClient interface`
  (params (newMember :type "Actor Object Reference") (`init?` :type Boolean)))

(fn `AddNewXpedMemOnServ interface`
  (params (`leader's ref` :type "Actor Object Reference")))

(fn `Apply Useable Item Interface`
  (params (`Use item info` :type "/Game/GameSystem/Structures/S_UseableItemEffects Structure")))

(fn `call change movement mode after climbing down interface`)

(fn `change ignore components interface`
  (params (obj :type "PrimitiveComponent Object Reference (by ref)") (value :type "Boolean (by ref)")))

(fn `Change Quest Dialog bool value interface`
  (params (value :type Boolean)))

(fn `char multicast animation interface`
  (params (`move mode` :type "EMovementMode Enum" :default "MOVE_None") (`play rate` :type "Float (double-precision)")))

(fn `Char Takes Dmg interface`
  (params (`Dmg In` :type Integer) (`KB Direction` :type Integer))
  (return))

(fn `Equip an Item Interface`
  (params (`pickup Item Info` :type "/Game/GameSystem/Structures/S_PickupItemInfo Structure") (index :type Integer)))

(fn `Gain EXP interface`
  (params (`Exp Amount` :type Integer)))

(fn `get AP points available interface`
  (returns (`points available` :type Integer))
  (return 0))

(fn `get char class interface`
  (returns (`char class` :type "/Game/GameSystem/Enums/E_ClassesAvailable Enum") (`class category` :type "/Game/GameSystem/Enums/E_ClassesCategories Enum"))
  (return "NewEnumerator29" "NewEnumerator0"))

(fn `get char Exp details interface`
  (returns (`max exp for curr lvl` :type Integer64) (`curr exp` :type Integer64))
  (return 0 0))

(fn `get char info for master platform or ladder interface`
  (returns (`atk anim in prog?` :type Boolean) (`char movement` :type "CharacterMovementComponent Object Reference") (`up key pressed?` :type Boolean) (`overlapping comp arr` :type "Array of ActorComponent Object Reference") (`capsule comp` :type "CapsuleComponent Object Reference") (`down key pressed?` :type Boolean))
  (return false null false _ null false))

(fn `get char LVL interface`
  (returns (level :type Integer))
  (return 0))

(fn `get char name interface`
  (returns (`char name` :type Name))
  (return "None"))

(fn `get chat bubble widget comp Interface`
  (returns (`chat bubble ref` :type "WidgetComponent Object Reference"))
  (return null))

(fn `Get dmg widget comp interface`
  (returns (`dmg widget comp ref` :type "WidgetComponent Object Reference"))
  (return null))

(fn `get Equip widget REF interface`
  (returns (`equip widget ref` :type "UserWidget Object Reference"))
  (return null))

(fn `get highest ever range interface`
  (returns (`min range` :type Integer) (`max range` :type Integer))
  (return 0 0))

(fn `get main widget interface`
  (returns (`main widget ref` :type "UserWidget Object Reference"))
  (return null))

(fn `get mapChanged bool interface`
  (returns (value :type Boolean))
  (return false))

(fn `get stats interface`
  (returns (`char stats` :type "/Game/GameSystem/Structures/CharactersStats_Struct Structure"))
  (return))

(fn `getPlayerState interface`
  (returns (`player'sState` :type "PlayerState Object Reference"))
  (return null))

(fn `InvitationREQ on client interface`
  (params (`Invitation TYPE` :type "/Game/GameSystem/Enums/E_NotificationWidgetTypes Enum" :default "NewEnumerator0") (`inviter's REF` :type "Actor Object Reference") (`inviter's name` :type Name)))

(fn `InvitationREQ via Server interface`
  (params (`invitation type` :type "/Game/GameSystem/Enums/E_NotificationWidgetTypes Enum" :default "NewEnumerator0") (`otherPlayer's REF` :type "Actor Object Reference")))

(fn `Is Attack Anim In Progress interface`
  (returns (value :type Boolean))
  (return false))

(fn `JoinExistingXpedition interface`
  (params (expeditionMembersArr :type "Array of Actor Object Reference") (`leader's REF` :type "Actor Object Reference")))

(fn `LogOut change expedition widget appearance interface`)

(fn `open other stats widget interface`
  (params (`other char ref` :type "Actor Object Reference"))
  (returns (`created widget ref` :type "UserWidget Object Reference") (`success?` :type Boolean))
  (return null false))

(fn `Ready to multicast speech bubble interface`
  (params (Duration :type "Float (double-precision)") (Msg :type Text)))

(fn `set climb bool value interface`
  (params (value :type Boolean)))

(fn `set expedition leader to all members interface`
  (params (newLeader :type "Actor Object Reference") (`old leader ref` :type "Actor Object Reference") (`old leaving?` :type Boolean) (`kick?` :type Boolean) (`mapChange?` :type Boolean) (`logOut?` :type Boolean)))

(fn `set other as expedition leader interface`
  (params (`new leader or kicked player REF` :type "Actor Object Reference") (`all Xped members` :type "Array of Actor Object Reference") (`old leader leaving?` :type Boolean) (`kick operation?` :type Boolean) (`mapChange?` :type Boolean) (logOut :type Boolean)))

(fn `set other player options widget interface`
  (params (`other char REF` :type "Actor Object Reference")))

(fn `set rakins interface`
  (params (`rakins info` :type "/Game/GameSystem/Structures/Rakins_Struct Structure")))

(fn `SetInvWidget interface`
  (params (`inv widget ref` :type "UserWidget Object Reference")))

(fn `setInXpeditionAndLeaderValues interface`
  (params (`inXpedition?` :type Boolean) (`isLeader?` :type Boolean) (membersAmnt :type Integer) (membersArr :type "Array of Actor Object Reference") (LeaderREF :type "Actor Object Reference")))

(fn `UnEquip Item interface`
  (params (`equip categ` :type "/Game/GameSystem/Enums/E_EquipmentCategories Enum" :default "NewEnumerator0") (`left glove?` :type Boolean) (`ring num` :type Integer) (`left earring?` :type Boolean))
  (returns (`can unequip?` :type Boolean))
  (return false))

(fn `update Focusable widget after close interface`
  (params (`widget to close` :type "UserWidget Object Reference")))

(fn `updateLvlTxtOnXpedWidgetClient interface`)