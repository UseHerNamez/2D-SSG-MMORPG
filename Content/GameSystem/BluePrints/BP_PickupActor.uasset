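; World item pickup that shows the item's sprite and exposes its ItemInformation and collision sphere.
; On BeginPlay the sprite launches under physics, with the sphere following by polling until it stops or starts to rotate, then physics turns off.
; Clients loop an eased bob, count down lifespan by timer and fade the sprite near expiry.
; Interface events make it fly to the collecting player while fading on clients, or destroy it.
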(event `self.ReceiveBeginPlay`
  (bind _icon_sprite (`self.Icon_Sprite`))
  (bind _icon_sprite_2 (`self.Icon_Sprite`))
  (bind _icon_sprite_3 (`self.Icon_Sprite`))
  (bind _icon_sprite_4 (`self.Icon_Sprite`))
  (bind _icon_sprite_5 (`self.Icon_Sprite`))
  (bind _returnvalue (<= (`self.LifeSpan`) 2.0))
  (bind _returnvalue_2 (`SceneComponent.K2_GetComponentLocation` _icon_sprite_5))
  (bind (_spritecolor_r _spritecolor_g _spritecolor_b) (break `LinearColor` (`PaperSpriteComponent.SpriteColor` _icon_sprite_3)))
  ;[1 1 1] Floating animation
  (`self.EventSetClientLifeSpan` (`self.GetLifeSpan`))
  (`PaperSpriteComponent.SetSprite` _icon_sprite_4 (`.SpriteOfTheTexture_51_26F6AB1D48E0EBC0D119538F6944E051` (break `/Game/GameSystem/Structures/Struct_ItemProperties` (`.ItemPropertiesStruct_14_60179F8943E4075BC3DE8680B21848D6` (break `/Game/GameSystem/Structures/S_PickupItemInfo` (`self.ItemInformation`))))))
  (`SceneComponent.K2_SetWorldLocation` _icon_sprite_4 (`SceneComponent.K2_GetComponentLocation` (`self.Sphere`)) false false)
  (`PrimitiveComponent.SetTranslucentSortPriority` _icon_sprite_4 30)
  (`PrimitiveComponent.SetSimulatePhysics` _icon_sprite_4 true)
  (`PrimitiveComponent.SetPhysicsLinearVelocity` _icon_sprite_2 (`KismetMathLibrary.MakeVector` (`self.HorizontalVelocity`) 0.0 400.0) true "None")
  (`PrimitiveComponent.SetEnableGravity` _icon_sprite_2 true)
  (if (not (`KismetMathLibrary.EqualExactly_VectorVector` (`SceneComponent.GetComponentVelocity` _icon_sprite_4))) :!label _label
    (`SceneComponent.K2_SetWorldLocation` (`self.Scene`) _returnvalue_2 false true)
    (`SceneComponent.K2_SetWorldLocation` (`self.Sphere`) _returnvalue_2 false true)
    (if (!= (`SceneComponent.K2_GetComponentRotation` _icon_sprite_4) (struct) :`ErrorTolerance` 0.0)
      (`SceneComponent.K2_SetWorldRotation` :`self` _icon_sprite_4 :`bTeleport` true)
      (else
        (`KismetSystemLibrary.Delay` 0.15)
        (goto _label))))
  (`PrimitiveComponent.SetEnableGravity` _icon_sprite_5 false)
  (`PrimitiveComponent.SetSimulatePhysics` _icon_sprite_5 false)
  (`SceneComponent.K2_SetWorldLocation` (`self.Scene`) _returnvalue_2 false true)
  (`SceneComponent.K2_SetWorldLocation` (`self.Sphere`) _returnvalue_2 false true)
  (`SceneComponent.K2_SetWorldLocation` _icon_sprite _returnvalue_2 false true)
  (`/Engine/EditorBlueprintResources/ActorMacros.Switch Has Authority`
    (:`Remote`
      (`KismetSystemLibrary.MoveComponentTo` _icon_sprite (+ _returnvalue_2 (0.0 0.0 5.0)) (struct) true true 0.8 :!label _label_2)
      (`KismetSystemLibrary.Delay` 0.6 :!label _label_3)
      (if (`self.FloatingLoop`)
        (set `self.FloatingLoop` false)
        (if _returnvalue
          (bind (_direction _newtrack_0 _fade_away_gradually) (`Timeline|Timeline_1` :!label _label_4)
            (:`Update`
              (`PaperSpriteComponent.SetSpriteColor` _icon_sprite_3 (make `LinearColor` _spritecolor_r _spritecolor_g _spritecolor_b (`KismetMathLibrary.Lerp` 0.0 1.0 _fade_away_gradually)))))
          (else
            (`KismetSystemLibrary.MoveComponentTo` _icon_sprite (- _returnvalue_2 (0.0 0.0 5.0)) (struct) true true 0.8 :!label _label_5)
            (goto _label_3)))
        (else
          (set `self.FloatingLoop` true)
          (if _returnvalue
            (goto _label_4)
            (else
              (goto _label_2))))))))

(event `EventSetClientLifeSpan`
  (params (LifeSpan :type "Float (double-precision)"))
  (`/Engine/EditorBlueprintResources/ActorMacros.Switch Has Authority`
    (:`Remote`
      (set `self.LifeSpan` LifeSpan)
      (bind _returnvalue (`KismetSystemLibrary.K2_SetTimerDelegate` (delegate `TimerEventSetClientLifeSpan`) 1.0 true))
      (set `self.LifeSpanTimeHandler` _returnvalue))))

(event `TimerEventSetClientLifeSpan`
  (set `self.LifeSpan` (- (`self.LifeSpan`) 1.0)))

(event `ChasePalyerWhenPickup`
  (params (`Player REF` :type "Character Object Reference (by ref)"))
  (`/Engine/EditorBlueprintResources/ActorMacros.Switch Has Authority`
    (:`Remote`
      (`|ExecutionSequence`
        (:`then_0`
          (goto _label_2 :!via `Stop`))
        (:`then_1`
          (goto _label_5 :!via `Stop`))
        (:`then_2`
          (bind (_direction _fade_away_gradually _opacity) (`Timeline|Timeline_2` :!via `PlayFromStart`)
            (:`Update`
              (`SceneComponent.K2_SetWorldLocation` (`self.Icon_Sprite`) (`KismetMathLibrary.VLerp` (`SceneComponent.K2_GetComponentLocation` (`self.Icon_Sprite`)) (`SceneComponent.K2_GetComponentLocation` (`Character.CapsuleComponent` `Player REF`)) _opacity) false false)
              (`PaperSpriteComponent.SetSpriteColor` (`self.Icon_Sprite`) (make `LinearColor` 1.0 1.0 1.0 (`KismetMathLibrary.Lerp` 0.1 1.0 _fade_away_gradually))))))))))

(event `/Game/GameSystem/BluePrints/BPInterface_PickupObjects.Chase player interface`
  (params (`Char ref` :type "Character Object Reference"))
  (`self.ChasePalyerWhenPickup` `Char ref`))

(event `SelfDestruct`
  (`self.K2_DestroyActor`))

(event `/Game/GameSystem/BluePrints/BPInterface_PickupObjects.self destruct interface`
  (`self.SelfDestruct`))

(fn `return collision bounds`
  (returns (`Sphere REF` :type "SphereComponent Object Reference"))
  (return (`self.Sphere`)))

(fn `return item info`
  (returns (`item info` :type "/Game/GameSystem/Structures/S_PickupItemInfo Structure") (`rakin info` :type "/Game/GameSystem/Structures/Rakins_Struct Structure"))
  (return (`self.ItemInformation`)))

(fn `UserConstructionScript`)