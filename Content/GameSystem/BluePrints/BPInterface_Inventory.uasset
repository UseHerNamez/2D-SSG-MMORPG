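; Blueprint Interface for the inventory system, declaring the calls other objects use to reach an inventory without direct casting.
; It covers adding, using, removing, moving, dropping and sorting items, with most slot calls taking an index and an array selector.
; It also exposes Rakins get and drop, character and widget references, and inventory visibility.
; All functions are signatures only; the sort call is named as server-side.
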(fn `activate drop an item func interface`
  (params (index :type Integer) (array :type "/Game/GameSystem/Enums/E_ItemCategories Enum" :default "NewEnumerator0") (`drop amt` :type Integer)))

(fn `activate drop rakins func interface`
  (params (`amnt to drop` :type "/Game/GameSystem/Structures/Rakins_Struct Structure")))

(fn `activate func try use item interface`
  (params (`item info` :type "/Game/GameSystem/Structures/S_PickupItemInfo Structure") (index :type Integer)))

(fn `activate On Drop func interface`
  (params (`from index` :type Integer) (`to index` :type Integer) (`which arr` :type "/Game/GameSystem/Enums/E_ItemCategories Enum" :default "NewEnumerator0")))

(fn `activate sort inventory func on serv Interface`
  (params (`which array` :type "/Game/GameSystem/Enums/E_ItemCategories Enum" :default "NewEnumerator0") (`reverse?` :type Boolean)))

(fn `add an item interface`
  (params (`notification?` :type Boolean) (`rakins info` :type "/Game/GameSystem/Structures/Rakins_Struct Structure") (`item info` :type "/Game/GameSystem/Structures/S_PickupItemInfo Structure")))

(fn `call change visible bool value func interface`
  (params (val :type Boolean)))

(fn `call hide inv func interface`)

(fn `call remove item at index interface`
  (params (index :type Integer) (amount :type Integer) (`which array` :type "/Game/GameSystem/Enums/E_ItemCategories Enum" :default "NewEnumerator0"))
  (returns (success :type Boolean))
  (return false))

(fn `Check Empty Slot And Amount Interface`
  (params (index :type Integer) (`which array` :type "/Game/GameSystem/Enums/E_ItemCategories Enum" :default "NewEnumerator0"))
  (returns (`is empty` :type Boolean) (amount :type Integer))
  (return false 0))

(fn `get array of inv slots data`
  (params (`which array` :type "/Game/GameSystem/Enums/E_ItemCategories Enum" :default "NewEnumerator0"))
  (returns (`inv slot data arr` :type "Array of /Game/GameSystem/Structures/S_InventorySlotData Structure"))
  (return))

(fn `get char ref (as paper) interface`
  (returns (`char ref` :type "PaperDoll2DCharacter Object Reference"))
  (return null))

(fn `get inv widget interface`
  (returns (`inv widget` :type "UserWidget Object Reference"))
  (return null))

(fn `get item info at index interface`
  (params (index :type Integer) (`which array` :type "/Game/GameSystem/Enums/E_ItemCategories Enum" :default "NewEnumerator0"))
  (returns (iteminfo :type "/Game/GameSystem/Structures/S_PickupItemInfo Structure") (amount :type Integer) (`empty?` :type Boolean))
  (return (struct) 0 false))

(fn `get main widget as user widget interface`
  (returns (`main widget ref` :type "UserWidget Object Reference"))
  (return null))

(fn `get rakins interface`
  (returns (rakins :type "/Game/GameSystem/Structures/Rakins_Struct Structure"))
  (return))

(fn `set inv widget`
  (params (`inv widget` :type "UserWidget Object Reference")))