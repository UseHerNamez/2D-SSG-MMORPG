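; Climbable ladder or rope actor for Paper2D characters, using a rope-top sprite when not a ladder.
; Bottom and top trigger overlaps, or the ChangeToClimbMode functions, check up/down input through BPInterface_Char.
; Climbing sets Flying movement, snaps and plane-constrains the character on X, and makes it ignore the overlapping FloatPlatform via interfaces.
; Leaving both triggers ends climbing and restores falling and default constraints; only top-trigger events are authority-gated.
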(event `self.ReceiveBeginPlay`
  (if (not (`self.Ladder?`))
    (`PaperSpriteComponent.SetSprite` (`self.TopRope`) "/Game/GameSystem/Textures/ObjectsInMap/TopRopePart_Sprite.TopRopePart_Sprite")))

(event `self.ClimbCollision.OnComponentBeginOverlap`
  (params (OverlappedComponent :type "PrimitiveComponent Object Reference") (OtherActor :type "Actor Object Reference") (OtherComp :type "PrimitiveComponent Object Reference") (OtherBodyIndex :type Integer) (bFromSweep :type Boolean) (SweepResult :type "HitResult Structure (by ref)"))
  (bind _returnvalue_x (`KismetMathLibrary.BreakVector` (`SceneComponent.K2_GetComponentLocation` (`self.ClimbCollision`))))
  (bind (_returnvalue_x_2 _returnvalue_y _returnvalue_z) (`KismetMathLibrary.BreakVector` (`SceneComponent.K2_GetComponentLocation` (`Actor.RootComponent` OtherActor))))
  (bind _output (`|GetArrayItem` (`PrimitiveComponent.GetOverlappingActors` (`self.Ladder or Rope`) "/Game/GameSystem/BluePrints/PlatformsBPs/WTJB_Map/FloatPlatform.FloatPlatform_C")))
  (bind (_atk_anim_in_prog_ _char_movement _overlapping_comp_arr _up_key_pressed_ _capsule_comp) (`self.check if actor uses char interface` OtherActor :!label _label))
  (if (not _atk_anim_in_prog_)
    (if _up_key_pressed_
      (message `/Game/GameSystem/BluePrints/BPInterface_Char.set climb bool value interface` OtherActor true)
      (if (`KismetSystemLibrary.IsValid` _output)
        (if (`KismetSystemLibrary.DoesImplementInterface` _output "/Game/GameSystem/BluePrints/BPInterface_Platforms.BPInterface_Platforms_C")
          (bind _platform (message `/Game/GameSystem/BluePrints/BPInterface_Platforms.get platform and collisions` _output))
          (message `/Game/GameSystem/BluePrints/BPInterface_Char.change ignore components interface` OtherActor _platform true)
          (`CharacterMovementComponent.SetMovementMode` _char_movement "MOVE_Flying" 0)
          (message `/Game/GameSystem/BluePrints/BPInterface_Char.I_callChangeAnimState` OtherActor "ClimbLadder")
          (`MovementComponent.StopMovementImmediately` _char_movement)
          (`MovementComponent.SetPlaneConstraintAxisSetting` _char_movement "X")
          (`SceneComponent.K2_SetWorldLocation` _capsule_comp (`KismetMathLibrary.MakeVector` _returnvalue_x 0.0 _returnvalue_z) false false)
          (`SceneComponent.K2_SetWorldLocation` (`Actor.RootComponent` OtherActor) (`KismetMathLibrary.MakeVector` _returnvalue_x 0.0 _returnvalue_z) false false)
          (`/Engine/EditorBlueprintResources/StandardMacros.DoOnce` false :!via `Reset` :!label _label_2
            (:`Completed`
              (goto _label)))
          (else
            (goto _label_2 :!via `Reset`)))
        (else
          (goto _label_2 :!via `Reset`)))
      (else
        (goto _label_2 :!via `Reset`)))
    (else
      (goto _label_2 :!via `Reset`))))

(event `self.ClimbCollision.OnComponentEndOverlap`
  (params (OverlappedComponent :type "PrimitiveComponent Object Reference") (OtherActor :type "Actor Object Reference") (OtherComp :type "PrimitiveComponent Object Reference") (OtherBodyIndex :type Integer))
  (bind _rootcomponent (`Actor.RootComponent` OtherActor))
  (bind (_returnvalue_x _returnvalue_y _returnvalue_z) (`KismetMathLibrary.BreakVector` (`SceneComponent.K2_GetComponentLocation` _rootcomponent)))
  (bind (_atk_anim_in_prog_ _char_movement) (`self.check if actor uses char interface` OtherActor))
  (if (not _atk_anim_in_prog_)
    (if (!= (`KismetArrayLibrary.Array_Find` (`self.GetOverlappingComponents` OtherActor) (`self.TopLadderCollisionBox`)) -1)
      (`SceneComponent.K2_SetWorldLocation` _rootcomponent (`KismetMathLibrary.MakeVector` _returnvalue_x 0.0 (+ _returnvalue_z 10.0)) false true)
      (else
        (message `/Game/GameSystem/BluePrints/BPInterface_Char.set climb bool value interface` OtherActor false)
        (if (not (`|EnumEquality` (`CharacterMovementComponent.MovementMode` _char_movement) "MOVE_Walking"))
          (`CharacterMovementComponent.SetMovementMode` _char_movement "MOVE_Falling" 0)
          (`MovementComponent.SetPlaneConstraintAxisSetting` _char_movement "UseGlobalPhysicsSetting"))))))

(event `self.TopLadderCollisionBox.OnComponentBeginOverlap`
  (params (OverlappedComponent :type "PrimitiveComponent Object Reference") (OtherActor :type "Actor Object Reference") (OtherComp :type "PrimitiveComponent Object Reference") (OtherBodyIndex :type Integer) (bFromSweep :type Boolean) (SweepResult :type "HitResult Structure (by ref)"))
  (bind _rootcomponent (`Actor.RootComponent` OtherActor))
  (bind _returnvalue_x (`KismetMathLibrary.BreakVector` (`SceneComponent.K2_GetComponentLocation` (`self.TopLadderCollisionBox`))))
  (bind (_returnvalue_x_2 _returnvalue_y _returnvalue_z) (`KismetMathLibrary.BreakVector` (`SceneComponent.K2_GetComponentLocation` _rootcomponent)))
  (bind _output (`|GetArrayItem` (`PrimitiveComponent.GetOverlappingActors` (`self.Ladder or Rope`) "/Game/GameSystem/BluePrints/PlatformsBPs/WTJB_Map/FloatPlatform.FloatPlatform_C")))
  (`/Engine/EditorBlueprintResources/ActorMacros.Switch Has Authority`
    (:`Authority`
      (bind (_atk_anim_in_prog_ _char_movement _overlapping_comp_arr _up_key_pressed_ _capsule_comp _down_key_pressed_) (`self.check if actor uses char interface` OtherActor))
      (if (and _down_key_pressed_ (not _atk_anim_in_prog_))
        (message `/Game/GameSystem/BluePrints/BPInterface_Char.set climb bool value interface` OtherActor true)
        (if (`KismetSystemLibrary.IsValid` _output)
          (if (`KismetSystemLibrary.DoesImplementInterface` _output "/Game/GameSystem/BluePrints/BPInterface_Platforms.BPInterface_Platforms_C")
            (bind _platform (message `/Game/GameSystem/BluePrints/BPInterface_Platforms.get platform and collisions` _output))
            (message `/Game/GameSystem/BluePrints/BPInterface_Char.change ignore components interface` OtherActor _platform true)
            (`CharacterMovementComponent.SetMovementMode` _char_movement "MOVE_Flying" 0)
            (message `/Game/GameSystem/BluePrints/BPInterface_Char.I_callChangeAnimState` OtherActor "ClimbLadder")
            (`MovementComponent.StopMovementImmediately` _char_movement)
            (`MovementComponent.SetPlaneConstraintAxisSetting` _char_movement "X")
            (`SceneComponent.K2_SetWorldLocation` _rootcomponent (`KismetMathLibrary.MakeVector` _returnvalue_x 0.0 (- _returnvalue_z 20.0)) false false)))))))

(event `self.TopLadderCollisionBox.OnComponentEndOverlap`
  (params (OverlappedComponent :type "PrimitiveComponent Object Reference") (OtherActor :type "Actor Object Reference") (OtherComp :type "PrimitiveComponent Object Reference") (OtherBodyIndex :type Integer))
  (`/Engine/EditorBlueprintResources/ActorMacros.Switch Has Authority`
    (:`Authority`
      (bind (_atk_anim_in_prog_ _char_movement _overlapping_comp_arr _up_key_pressed_ _capsule_comp) (`self.check if actor uses char interface` OtherActor))
      (`PrimitiveComponent.SetCollisionEnabled` _capsule_comp "QueryAndPhysics")
      (if (not _atk_anim_in_prog_)
        (if (not (!= (`KismetArrayLibrary.Array_Find` (`self.GetOverlappingComponents` OtherActor) (`self.ClimbCollision`)) -1))
          (bind _movementmode (`CharacterMovementComponent.MovementMode` _char_movement))
          (if (not (or (`|EnumEquality` _movementmode "MOVE_Walking") (`|EnumEquality` _movementmode "MOVE_Falling")))
            (`CharacterMovementComponent.SetMovementMode` _char_movement "MOVE_Falling" 0))
          (message `/Game/GameSystem/BluePrints/BPInterface_Char.set climb bool value interface` OtherActor false)
          (`MovementComponent.SetPlaneConstraintAxisSetting` _char_movement "UseGlobalPhysicsSetting"))))))

(event `self.Ladder or Rope.OnComponentBeginOverlap`
  (params (OverlappedComponent :type "PrimitiveComponent Object Reference") (OtherActor :type "Actor Object Reference") (OtherComp :type "PrimitiveComponent Object Reference") (OtherBodyIndex :type Integer) (bFromSweep :type Boolean) (SweepResult :type "HitResult Structure (by ref)"))
  (bind _output (`|GetArrayItem` (`PrimitiveComponent.GetOverlappingActors` (`self.Ladder or Rope`) "/Game/GameSystem/BluePrints/PlatformsBPs/WTJB_Map/FloatPlatform.FloatPlatform_C")))
  (bind _atk_anim_in_prog_ (`self.check if actor uses char interface` OtherActor))
  (if (not _atk_anim_in_prog_)
    (if (`KismetSystemLibrary.IsValid` _output)
      (if (`KismetSystemLibrary.DoesImplementInterface` _output "/Game/GameSystem/BluePrints/BPInterface_Platforms.BPInterface_Platforms_C")
        (bind _platform (message `/Game/GameSystem/BluePrints/BPInterface_Platforms.get platform and collisions` _output))
        (message `/Game/GameSystem/BluePrints/BPInterface_Char.change ignore components interface` OtherActor _platform true)))))

(fn `ChangeToClimbModeDown`
  (params (Char :type "Character Object Reference"))
  (bind _returnvalue_x (`KismetMathLibrary.BreakVector` (`SceneComponent.K2_GetComponentLocation` (`self.TopLadderCollisionBox`))))
  (bind _output (`|GetArrayItem` (`self.GetOverlappingActors` "/Game/GameSystem/BluePrints/PlatformsBPs/WTJB_Map/FloatPlatform.FloatPlatform_C")))
  (bind (_atk_anim_in_prog_ _char_movement _overlapping_comp_arr _up_key_pressed_ _capsule_comp _down_key_pressed_) (`self.check if actor uses char interface` Char))
  (if (!= (`KismetArrayLibrary.Array_Find` (`PrimitiveComponent.GetOverlappingActors` (`self.TopLadderCollisionBox`) "/Script/Paper2D.PaperCharacter") Char) -1)
    (if _down_key_pressed_
      (`CharacterMovementComponent.SetMovementMode` _char_movement "MOVE_Flying" 0)
      (message `/Game/GameSystem/BluePrints/BPInterface_Char.set climb bool value interface` Char true)
      (if (`KismetSystemLibrary.IsValid` _output)
        (if (`KismetSystemLibrary.DoesImplementInterface` _output "/Game/GameSystem/BluePrints/BPInterface_Platforms.BPInterface_Platforms_C")
          (bind _platform (message `/Game/GameSystem/BluePrints/BPInterface_Platforms.get platform and collisions` _output))
          (message `/Game/GameSystem/BluePrints/BPInterface_Char.change ignore components interface` Char _platform true)
          (`MovementComponent.SetPlaneConstraintAxisSetting` _char_movement "X")
          (bind (_returnvalue_x_2 _returnvalue_y _returnvalue_z) (`KismetMathLibrary.BreakVector` (`SceneComponent.K2_GetComponentLocation` _capsule_comp)))
          (`SceneComponent.K2_SetWorldLocation` _capsule_comp (`KismetMathLibrary.MakeVector` _returnvalue_x 0.0 (- _returnvalue_z 20.0)) false false)
          (return)))
      (else
        (return)))
    (else
      (return))))

(fn `ChangeToClimbModeUp`
  (params (Character :type "Character Object Reference"))
  (bind _returnvalue_x (`KismetMathLibrary.BreakVector` (`SceneComponent.K2_GetComponentLocation` (`self.ClimbCollision`))))
  (bind _output (`|GetArrayItem` (`PrimitiveComponent.GetOverlappingActors` (`self.Ladder or Rope`) "/Game/GameSystem/BluePrints/PlatformsBPs/WTJB_Map/FloatPlatform.FloatPlatform_C")))
  (bind (_atk_anim_in_prog_ _char_movement _overlapping_comp_arr _up_key_pressed_ _capsule_comp) (`self.check if actor uses char interface` Character))
  (if (!= (`KismetArrayLibrary.Array_Find` (`PrimitiveComponent.GetOverlappingActors` (`self.ClimbCollision`) "/Script/Paper2D.PaperCharacter") Character) -1)
    (if _up_key_pressed_
      (`CharacterMovementComponent.SetMovementMode` _char_movement "MOVE_Flying" 0)
      (message `/Game/GameSystem/BluePrints/BPInterface_Char.set climb bool value interface` Character true)
      (if (`KismetSystemLibrary.IsValid` _output)
        (if (`KismetSystemLibrary.DoesImplementInterface` _output "/Game/GameSystem/BluePrints/BPInterface_Platforms.BPInterface_Platforms_C")
          (bind _platform (message `/Game/GameSystem/BluePrints/BPInterface_Platforms.get platform and collisions` _output))
          (message `/Game/GameSystem/BluePrints/BPInterface_Char.change ignore components interface` Character _platform true))
        (`MovementComponent.StopMovementImmediately` _char_movement)
        (`MovementComponent.SetPlaneConstraintAxisSetting` _char_movement "X")
        (bind (_returnvalue_x_2 _returnvalue_y _returnvalue_z) (`KismetMathLibrary.BreakVector` (`SceneComponent.K2_GetComponentLocation` _capsule_comp)))
        (`SceneComponent.K2_SetWorldLocation` _capsule_comp (`KismetMathLibrary.MakeVector` _returnvalue_x 0.0 _returnvalue_z) false false)
        (return))
      (else
        (return)))
    (else
      (return))))

(fn `UserConstructionScript`)