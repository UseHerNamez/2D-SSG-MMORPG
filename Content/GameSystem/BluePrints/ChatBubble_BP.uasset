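; Chat bubble actor that shows a text message in a widget tied to a Paper character and hides it after a set duration.
; First run creates the widget and optionally assigns it in screen space to the character's widget component; later calls update its text through BubbleWidget_BPI.
; Each update restarts the hide timer.
; Location updates move the character's widget component on the X/Z plane.
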(event `/Game/GameSystem/BluePrints/BPInterface_SpeechBubbleBP.set vars interface`
  (params (txt :type Text) (`set comps?` :type Boolean) (`paper char ref` :type "Character Object Reference"))
  (bind _bubble_widget (`self.bubble Widget`))
  (set `self.Text` txt)
  (set `self.SetComponents?` `set comps?`)
  (set `self.paperCharREF` `paper char ref`)
  (`KismetSystemLibrary.K2_SetTimerDelegate` (delegate `bubbleDisAppear`) (`self.VisibleDuration`) :!label _label)
  (if (`self.just created?`)
    (set `self.just created?` false)
    (bind _returnvalue (`|CreateWidget` "/Game/GameSystem/Widgets/ChatBubbleWidget.ChatBubbleWidget_C" null (`self.Text`) self))
    (set `self.bubble Widget` _returnvalue)
    (if (`self.SetComponents?`)
      (bind _chat_bubble_ref (message `/Game/GameSystem/BluePrints/BPInterface_Char.get chat bubble widget comp Interface` (`self.paperCharREF`)))
      (`WidgetComponent.SetWidget` _chat_bubble_ref _returnvalue)
      (`WidgetComponent.SetWidgetSpace` _chat_bubble_ref "Screen"))
    (elif (`KismetSystemLibrary.DoesImplementInterface` _bubble_widget "/Game/BubbleWidget_BPI.BubbleWidget_BPI_C")
      (message `/Game/BubbleWidget_BPI.Set text interface` _bubble_widget (`self.Text`)))))

(event `self.ReceiveBeginPlay`
  (goto _label))

(event `bubbleDisAppear`
  (bind _bubble_widget (`self.bubble Widget`))
  (if (`KismetSystemLibrary.DoesImplementInterface` _bubble_widget "/Game/BubbleWidget_BPI.BubbleWidget_BPI_C")
    (message `/Game/BubbleWidget_BPI.HideBubble interface` _bubble_widget)
    (else
      (`KismetSystemLibrary.PrintString` "no impl widget bpi"))))

(event `/Game/GameSystem/BluePrints/BPInterface_SpeechBubbleBP.set location interface`
  (params (X :type "Float (single-precision)") (Y :type "Float (single-precision)"))
  (`self.Set location` (`KismetMathLibrary.MakeVector2D` X Y)))

(fn `get Player locally owns the bubble`
  (returns (Char :type "Character Object Reference"))
  (return (`self.paperCharREF`)))

(fn `Set location`
  (params (Location :type "Vector2D Structure"))
  (bind _chat_bubble_ref (message `/Game/GameSystem/BluePrints/BPInterface_Char.get chat bubble widget comp Interface` (`self.paperCharREF`)))
  (`SceneComponent.K2_SetWorldLocation` _chat_bubble_ref (`KismetMathLibrary.MakeVector` Location_X 0.0 Location_Y) false false)
  (return))

(fn `UserConstructionScript`)