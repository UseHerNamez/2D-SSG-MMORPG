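; DmgSkin_BP is a damage number actor that displays a damage amount styled by a named damage skin.
; On BeginPlay it creates a DMG_Numbers_Widget, passing the skin name, amount and a reference to itself.
; Its Widget component hosts that widget in screen space, positioned using the root's world X and Z.
; A note states that monster hits always use the default skin with no crit.
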(event `self.ReceiveBeginPlay`
  (bind _widget (`self.Widget`))
  (bind _returnvalue (`|CreateWidget` "/Game/GameSystem/Widgets/DMG_Numbers_Widget.DMG_Numbers_Widget_C" null (`self.dmgSkinName`) (`self.dmgAmount`) self)) ; dmg skin will always be default when a monster hits, no crit too
  (`WidgetComponent.SetWidget` _widget _returnvalue)
  (`WidgetComponent.SetWidgetSpace` _widget "Screen")
  (`SceneComponent.K2_SetWorldLocation` _widget (`KismetMathLibrary.MakeVector` (.x (`SceneComponent.K2_GetComponentLocation` (`self.DefaultSceneRoot`))) 0.0 (.z (`SceneComponent.K2_GetComponentLocation` (`self.DefaultSceneRoot`)))) false false))

(fn `UserConstructionScript`)