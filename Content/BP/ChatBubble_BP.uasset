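; Chat bubble actor that shows a text message through a character's widget component for a limited time.
; On BeginPlay it sets its lifespan from VisibleDuration, creates a bubble widget with the text and a self reference, and assigns it to the character's component in screen space.
; SetLocation moves that component in world space, mapping the input's X and Y onto world X and Z.
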(event `self.ReceiveBeginPlay`
  (bind _chatbubblewidget (`/Game/2DSideScrollerBP/Blueprints/2DSideScrollerCharacter.ChatBubbleWidget` (`self.Char REF`)))
  (`self.SetLifeSpan` (`self.VisibleDuration`))
  (bind _returnvalue (`|CreateWidget` "/Game/GameSystem/Widgets/ChatBubbleWidget.ChatBubbleWidget_C" null (`self.Text`) self))
  (`WidgetComponent.SetWidget` _chatbubblewidget _returnvalue)
  (`WidgetComponent.SetWidgetSpace` _chatbubblewidget "Screen"))

(fn `Set location`
  (params (Location :type "Vector2D Structure"))
  (`SceneComponent.K2_SetWorldLocation` (`/Game/2DSideScrollerBP/Blueprints/2DSideScrollerCharacter.ChatBubbleWidget` (`self.Char REF`)) (`KismetMathLibrary.MakeVector` Location_X 0.0 Location_Y) false false)
  (return))

(fn `UserConstructionScript`)